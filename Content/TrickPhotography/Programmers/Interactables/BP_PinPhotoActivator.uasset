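; Interactable wall pin point that activates when an acceptable photo is pinned to it, showing dialog for success, failure or no photo.
; If an object is required, the photo must match the required filter and object class; otherwise any valid photo passes.
; Rejected photos are detached and pushed off along the actor's forward vector.
; An overlap volume tells the player character which actor class to look for in photos while inside.
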(event OnComponentBeginOverlap(IfRequireSpecialAndPlayerInThisCheckForActorInPhoto)
  (params (OverlappedComponent :type Primitive%20Component%20Object%20Reference) (OtherActor :type Actor%20Object%20Reference) (OtherComp :type Primitive%20Component%20Object%20Reference) (OtherBodyIndex :type Integer) (bFromSweep :type Boolean) (SweepResult :type Hit%20Result%20Structure%20%28by%20ref%29))
  (if (Variables|Default|GetbRequireObjectInPhoto)
    (bind _asbp_main_character (Utilities|Casting|CastToBP_MainCharacter OtherActor))
    (Default|InAreaOfSpecificPhotoObjects _asbp_main_character (Variables|Default|GetActorToLookFor) true)))

(event OnComponentEndOverlap(IfRequireSpecialAndPlayerInThisCheckForActorInPhoto)
  (params (OverlappedComponent :type Primitive%20Component%20Object%20Reference) (OtherActor :type Actor%20Object%20Reference) (OtherComp :type Primitive%20Component%20Object%20Reference) (OtherBodyIndex :type Integer))
  (if (Variables|Default|GetbRequireObjectInPhoto)
    (bind _asbp_main_character (Utilities|Casting|CastToBP_MainCharacter OtherActor))
    (Default|InAreaOfSpecificPhotoObjects _asbp_main_character 0 false)))

(event Custom|PhotoPinned
  (params (PhotoPinned :type BP%20Photograph%20Object%20Reference))
  (Utilities|IsValid PhotoPinned
    (:Is%20Valid
      (if (Variables|Default|GetbRequireObjectInPhoto)
        (if (Utilities|Enum|Equal(Enum) (Variables|/Game/TrickPhotography/Programmers/Core/Camera/BP_Photograph.BP_Photograph_C|GetFilterType PhotoPinned) (Variables|Default|GetRequiredFilter))
          (if (== (Variables|/Game/TrickPhotography/Programmers/Core/Camera/BP_Photograph.BP_Photograph_C|GetClassInPhoto PhotoPinned) (Variables|Default|GetActorToLookFor))
            (CallFunction|Activate :!label _label)
            (Default|SetDialogText (Variables|Default|GetUIRef) (Variables|Default|GetCompleteDialog) 5.0)
            (Utilities|FlowControl|Delay 5.0)
            (Default|SetDialogText (Variables|Default|GetUIRef) (Variables|Default|GetPostCompleteHint) 5.0)
            (else
              (Default|SetDialogText (Variables|Default|GetUIRef) (Variables|Default|GetFailDialog2) 5.0)
              (Utilities|FlowControl|Delay 0.5 :!label _label_2)
              (Default|SetAttachedtoWall PhotoPinned false)
              (Physics|AddForce (Variables|/Game/TrickPhotography/Programmers/Core/Camera/BP_Photograph.BP_Photograph_C|GetPhotograph PhotoPinned) (* (Transformation|GetActorForwardVector) 1e+04) "None" false)))
          (else
            (Default|SetDialogText (Variables|Default|GetUIRef) (Variables|Default|GetFailDialog) 5.0)
            (goto _label_2)))
        (else
          (goto _label))))
    (:Is%20Not%20Valid
      (Default|SetDialogText (Variables|Default|GetUIRef) (Variables|Default|GetBaseDialog) 5.0))))

(event EventBeginPlay
  (bind _staticmesh (Variables|Default|GetStaticMesh))
  (bind _returnvalue (Transformation|GetWorldTransform _staticmesh))
  (|CallParentFunction)
  (Variables|Default|SetPlacePos (Math|Transform|MakeTransform (.location _returnvalue) (.rotation _returnvalue) "1.000000,1.000000,1.000000"))
  (bind _asmain_player_controller (Utilities|Casting|CastToMainPlayerController (Game|GetPlayerController 0)))
  (Variables|Default|SetUIRef (Variables|/Game/TrickPhotography/Programmers/Core/Player/MainPlayerController.MainPlayerController_C|GetUIRef _asmain_player_controller)))

(fn ConstructionScript
  (|CallParentFunction))