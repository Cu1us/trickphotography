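; Interactable piece of a sequence puzzle that non-Cammy players press, reporting itself to PuzzleMainObject.
; The glow decal follows the puzzle's fail state, and completion marks the pressed piece as permanently activated.
; UpdateActivatedStatus swaps glow materials and toggles linked objects through BPI_Activatable or visibility, flickering via a delayable loop on failure before resetting.
; Pieces flagged IsEndAndMoai switch to the moai idol mesh and materials at BeginPlay.
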(event Custom|SetDecal
  (params (bGlow :type Boolean))
  (Rendering|SetActorHiddenInGame (Variables|Default|GetDecalStatueGlow) (not bGlow)))

(event Custom|UpdateActivatedStatus
  (params (bFailed :type Boolean) (bSetActivated :type Boolean))
  (if bFailed
    (Utilities|DelayableforLoop 0 5 :!label _label
      (:LoopBody
        (CallFunction|SetMaterial (Variables|Default|GetMaterialToUse))
        (Utilities|FlowControl|Delay 0.2)
        (CallFunction|SetMaterial (Variables|Default|GetMaterialToUseGlow))
        (Utilities|FlowControl|Delay 0.1)
        (goto _label CountUp))
      (:Completed
        (CallFunction|SetMaterial (Variables|Default|GetMaterialToUse))
        (Variables|Default|SetbActivatedTemporarily false)
        (CallFunction|UpdateActivatedStatus false false)))
    (else
      (bind _output_get (Variables|Default|SetbActivatedTemporarily bSetActivated))
      (if _output_get
        (CallFunction|SetMaterial (Variables|Default|GetMaterialToUseGlow))
        (for _array_element (Variables|Default|GetObjectsToActivateWhenActivated)
          (bind _asbpi_activatable (Utilities|Casting|CastToBPI_Activatable _array_element)
            (:then
              (Default|Activate _asbpi_activatable))
            (:CastFailed
              (Rendering|SetActorHiddenInGame _array_element false))))
        (else
          (CallFunction|SetMaterial (Variables|Default|GetMaterialToUse))
          (for _array_element_2 (Variables|Default|GetObjectsToActivateWhenActivated)
            (bind _asbpi_activatable_2 (Utilities|Casting|CastToBPI_Activatable _array_element_2)
              (:then
                (Default|Deactivate _asbpi_activatable_2))
              (:CastFailed
                (Rendering|SetActorHiddenInGame _array_element_2 true))))
          (CallFunction|SetDecal false))))))

(event EventBeginPlay
  (bind _filterstaticmesh (Variables|Default|GetFilterStaticMesh))
  (CallFunction|UpdateActivatedStatus false false)
  (CallFunction|SetDecal false)
  (if (Variables|Default|GetbIsEndAndMoai)
    (bind _output_get (Variables|Default|SetMeshToUse "/Game/TrickPhotography/Art/Enviroment/Meshes/S_idol_moai.S_idol_moai"))
    (Components|StaticMesh|SetStaticMesh _filterstaticmesh _output_get)
    (Variables|Default|SetMaterialToUseGlow "/Game/TrickPhotography/Art/Materials/Idols/M_Idol1glow.M_Idol1glow")
    (bind _output_get_2 (Variables|Default|SetMaterialToUse "/Game/TrickPhotography/Art/Materials/Idols/M_Idol1.M_Idol1"))
    (Class|FilterStaticMeshComponent|SetMainMaterial _filterstaticmesh _output_get_2)))

(event EventHoverEnd
  (params (HeldItem :type Pickupable%20Interface%20Interface) (bIsCammy :type Boolean))
  (Class|FilterActor|SetPPMHighlight "None"))

(event EventInteractStart
  (params (HeldItem :type Pickupable%20Interface%20Interface) (bIsCammy :type Boolean) (HitComponent :type Primitive%20Component%20Object%20Reference))
  (bind _puzzlemainobject (Variables|Default|GetPuzzleMainObject))
  (if (not bIsCammy)
    (if (not (Variables|Default|GetbActivatedTemporarily))
      (Audio|PlaySoundatLocation "/Game/TrickPhotography/Audio/Metasounds/MS_ButtonClick.MS_ButtonClick" (Transformation|GetActorLocation) "0, 0, 0" 1.0 1.0 0.0 0 0 0 0)
      (Utilities|IsValid _puzzlemainobject
        (:Is%20Valid
          (Default|ObjectInteractedwith _puzzlemainobject self)
          (CallFunction|SetDecal (not (Variables|/Game/TrickPhotography/Programmers/Interactables/BP_SequencePuzzleStart.BP_SequencePuzzleStart_C|GetbPuzzleHasFailed _puzzlemainobject)))
          (if (Variables|/Game/TrickPhotography/Programmers/Interactables/BP_SequencePuzzleStart.BP_SequencePuzzleStart_C|GetbPuzzleCompleted _puzzlemainobject)
            (Variables|Default|SetbActivatedForReal true)))))))

(fn ConstructionScript)

(fn SetMaterial
  (params (Mat :type Material%20Instance%20Object%20Reference))
  (Rendering|Material|SetMaterial (Variables|Default|GetFilterStaticMesh) 0 Mat)
  (Class|FilterStaticMeshComponent|SetMainMaterial (Variables|Default|GetFilterStaticMesh) Mat))

(fn GetInteractionType
  (params (bIsCammy :type Boolean) (HitComponent :type Primitive%20Component%20Object%20Reference))
  (return "NewEnumerator2" ""))

(fn HoverOngoing
  (params (HeldItem :type Pickupable%20Interface%20Interface) (HitComponent :type Primitive%20Component%20Object%20Reference))
  (return false))

(fn HoverStart
  (params (HeldItem :type Pickupable%20Interface%20Interface) (HitComponent :type Primitive%20Component%20Object%20Reference) (bIsCammy :type Boolean))
  (Class|FilterActor|SetPPMHighlight "HighlightPickup")
  (return false))