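; BP_KnockablePillar is a one-time interactable pillar that the player knocks over to release a Polaroid pack.
; On BeginPlay it spawns a BP_PolaroidPack with a filter unlock and thermal tutorial material, attached to a skeletal mesh socket with physics off.
; Interacting changes the pillar's collision object type, plays the fall animation, then enables pack physics after a delay.
; The "BONK IT!" tooltip shows only until the pillar falls.
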(event EventBeginPlay
  (bind _returnvalue (Game|SpawnActorfromClass "/Game/TrickPhotography/Programmers/Pickups/BP_PolaroidPack.BP_PolaroidPack_C" (Transformation|GetWorldTransform (Variables|Default|GetPolaroidPos)) "Undefined" "MultiplyWithRoot" 0 0))
  (Transformation|AttachComponentToComponent _returnvalue (Variables|Default|GetPillarSkeletalMesh) "PolaroidSocket" "KeepWorld" "KeepWorld" "KeepWorld" true)
  (Physics|SetSimulatePhysics (Variables|/Game/TrickPhotography/Programmers/Pickups/BP_PolaroidPack.BP_PolaroidPack_C|GetPack _returnvalue) false)
  (Variables|/Game/TrickPhotography/Programmers/Pickups/BP_PolaroidPack.BP_PolaroidPack_C|SetFilterToUnlock _returnvalue "NewEnumerator1")
  (Variables|/Game/TrickPhotography/Programmers/Pickups/BP_PolaroidPack.BP_PolaroidPack_C|SetTutorialMat _returnvalue "/Game/TrickPhotography/Art/Enviroment/Materials_MeshSpecific/Photograph/M_Thermal_Tutorial.M_Thermal_Tutorial"))

(event EventHoverEnd
  (params (HeldItem :type Pickupable%20Interface%20Interface) (bIsCammy :type Boolean)))

(event EventInteractStart
  (params (HeldItem :type Pickupable%20Interface%20Interface) (bIsCammy :type Boolean) (HitComponent :type Primitive%20Component%20Object%20Reference))
  (if (not (Variables|Default|GetKnockedOver))
    (Variables|Default|SetKnockedOver true)
    (Collision|SetCollisionObjectType (Variables|Default|GetPillarSkeletalMesh) "ECC_Pawn")
    (Components|Animation|PlayAnimation (Variables|Default|GetPillarSkeletalMesh) "/Game/TrickPhotography/Art/Enviroment/Meshes/PillarFallMontage.PillarFallMontage" false)
    (Utilities|FlowControl|Delay 1.7)
    (Physics|SetSimulatePhysics (Variables|/Game/TrickPhotography/Programmers/Pickups/BP_PolaroidPack.BP_PolaroidPack_C|GetPack (stale EventBeginPlay _returnvalue)) true)))

(fn ConstructionScript)

(fn GetInteractionType
  (params (bIsCammy :type Boolean) (HitComponent :type Primitive%20Component%20Object%20Reference))
  (if (Variables|Default|GetKnockedOver)
    (return "NewEnumerator0" "")
    (else
      (return "NewEnumerator2" "BONK IT!"))))

(fn HoverOngoing
  (params (HeldItem :type Pickupable%20Interface%20Interface) (HitComponent :type Primitive%20Component%20Object%20Reference))
  (return false))

(fn HoverStart
  (params (HeldItem :type Pickupable%20Interface%20Interface) (HitComponent :type Primitive%20Component%20Object%20Reference) (bIsCammy :type Boolean))
  (return false))