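; BP_DestructiblePot is a breakable puzzle prop built on a Chaos geometry collection, with its model swappable per instance through the construction script.
; On the first Chaos break event only, guarded by a Broken flag, it spawns a configurable object at the break location.
; The same event plays a break sound and starts a camera shake at a configurable intensity.
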(event OnChaosBreakEvent(Pot)
  (params (BreakEvent :type Chaos%20Break%20Event%20Structure%20%28by%20ref%29))
  (if (not (Variables|Default|GetbBroken))
    (Variables|Default|SetbBroken true)
    (Development|PrintString "it broke, wahoo")
    (Game|SpawnActorfromClass (Variables|Default|GetObjectToSpawn) (Math|Transform|MakeTransform (.location BreakEvent) "0, 0, 0" "1.000000,1.000000,1.000000") "AlwaysSpawn" "MultiplyWithRoot" 0 0)
    (Audio|Components|Audio|Play (Variables|Default|GetBreakSound) 0.2)
    (CameraShakes|StartCameraShake (Variables|Default|GetCameraShakeSource) "/Game/TrickPhotography/Programmers/Interactables/BP_CameraShake.BP_CameraShake_C" (Variables|Default|GetCameraShakeIntensity) "CameraLocal" "0, 0, 0")))

(fn ConstructionScript
  (bind _model (Variables|Default|GetModel))
  (Utilities|IsValid _model
    (:Is%20Valid
      (Class|GeometryCollectionComponent|SetRestCollection (Variables|Default|GetPot) _model false))))