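; Puzzle generator for a still life that spins up when its activator turns on and fires a beam to a given position for a final reveal.
; The Spin timeline drives rotation speed, whirring audio and orb material data, reversing on deactivation.
; TriggerReveal plays a FinalReveal timeline that adds extra spin and brightens the beam, then winds down and fades the sound.
; Tick rotates the ring part and tumbles the orb using sine and cosine of game time.
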(event Custom|TriggerReveal
  (params (Position :type Vector))
  (bind _beam (Variables|Default|GetBeam))
  (bind _whirring (Variables|Default|GetWhirring))
  (Utilities|FlowControl|Sequence
    (:then_0
      (bind _spinspeed (Timeline|FinalReveal Play)
        (:Update
          (Variables|Default|SetFinalRevealSpin (* _spinspeed 1.08e+03))
          (Rendering|Material|SetCustomPrimitiveDataFloat (Variables|Default|GetLittleOrb) 1 _spinspeed)
          (Niagara|SetNiagaraVariable(LinearColor) (Variables|Default|GetBeam) "Color" (Utilities|Struct|MakeLinearColor 1.0 1.0 1.0 _spinspeed)))
        (:Finished
          (bind (_direction _spinspeed_2 _soundpitch _soundvolume) (Timeline|Spin Reverse)
            (:Update
              (Variables|Default|SetActivationProgress _spinspeed_2)
              (Variables|Default|SetSpinSpeed (* (Variables|Default|GetMaxSpinSpeed) _spinspeed_2))
              (Audio|Components|Audio|SetPitchMultiplier _whirring _soundpitch)
              (Audio|Components|Audio|SetVolumeMultiplier _whirring _soundvolume :!class /Script/Engine.AudioComponent)
              (Rendering|Material|SetCustomPrimitiveDataFloat (Variables|Default|GetLittleOrb) 0 _spinspeed_2))))))
    (:then_1
      (Class|NiagaraComponent|SetVariablePosition _beam "End" Position)
      (Components|Activation|Activate _beam false)
      (Utilities|FlowControl|Delay 5.0)
      (Audio|Components|Audio|FadeOut (Variables|Default|GetWhirring) 3.0 0.0 "Linear" :!class /Script/Engine.AudioComponent))))

(event EventActivate
  (bind _whirring (Variables|Default|GetWhirring))
  (Audio|Components|Audio|Play (Variables|Default|GetWhirring) 0.0)
  (bind (_direction _spinspeed _soundpitch _soundvolume) (Timeline|Spin Play)
    (:Update
      (Variables|Default|SetActivationProgress _spinspeed)
      (Variables|Default|SetSpinSpeed (* (Variables|Default|GetMaxSpinSpeed) _spinspeed))
      (Audio|Components|Audio|SetPitchMultiplier _whirring _soundpitch)
      (Audio|Components|Audio|SetVolumeMultiplier _whirring _soundvolume :!class /Script/Engine.AudioComponent)
      (Rendering|Material|SetCustomPrimitiveDataFloat (Variables|Default|GetLittleOrb) 0 _spinspeed))))

(event EventDeactivate
  (bind _whirring (Variables|Default|GetWhirring))
  (Audio|Components|Audio|Stop (Variables|Default|GetWhirring))
  (bind (_direction _spinspeed _soundpitch _soundvolume) (Timeline|Spin Reverse)
    (:Update
      (Variables|Default|SetActivationProgress _spinspeed)
      (Variables|Default|SetSpinSpeed (* (Variables|Default|GetMaxSpinSpeed) _spinspeed))
      (Audio|Components|Audio|SetPitchMultiplier _whirring _soundpitch)
      (Audio|Components|Audio|SetVolumeMultiplier _whirring _soundvolume :!class /Script/Engine.AudioComponent)
      (Rendering|Material|SetCustomPrimitiveDataFloat (Variables|Default|GetLittleOrb) 0 _spinspeed))))

(event EventTick
  (params (DeltaSeconds :type Float%20%28single-precision%29))
  (bind _returnvalue (Utilities|Time|GetGameTimeinSeconds))
  (bind _spinspeed (Variables|Default|GetSpinSpeed))
  (bind _finalrevealspin (Variables|Default|GetFinalRevealSpin))
  (bind _returnvalue_2 (* DeltaSeconds _spinspeed))
  (bind _returnvalue_3 (* _finalrevealspin DeltaSeconds))
  (bind _returnvalue_4 (+ _returnvalue_2 _returnvalue_3))
  (bind _returnvalue_5 (* _returnvalue_4 0.5))
  (Transformation|AddLocalRotation (Variables|Default|GetRotatingPart) (Math|Rotator|MakeRotator 0.0 0.0 _returnvalue_4) false false)
  (Transformation|AddWorldRotation (Variables|Default|GetLittleOrb) (Math|Rotator|MakeRotator _returnvalue_5 (* _returnvalue_5 (Math|Trig|Sin(Radians) _returnvalue)) (* _returnvalue_5 (Math|Trig|Cos(Radians) _returnvalue))) false false))

(event EventBeginPlay
  (bind _activator (Variables|Default|GetActivator))
  (EventDispatchers|BindEventtoOnActivated _activator (delegate EventActivate))
  (EventDispatchers|BindEventtoOnDeactivated _activator (delegate EventDeactivate)))

(fn ConstructionScript)