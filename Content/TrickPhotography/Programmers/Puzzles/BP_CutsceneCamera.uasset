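; BP_CutsceneCamera is a possessable cutscene camera that flies along a track, optionally playing a jingle.
; Activate has the player controller possess it, then Tick advances time, remapped by AnimationCurve, to place the camera on the track.
; Rotation stays static, looks at an optional FocusPoint or follows the track.
; After an end delay, or on skip input while animating, it signals completion and repossesses the main character.
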(event Input|EnhancedActionEvents|EnhancedInputActionIA_SkipCutscene
  (params (ActionValue :type Boolean) (ElapsedSeconds :type Float%20%28double-precision%29) (TriggeredSeconds :type Float%20%28double-precision%29) (InputAction :type Input%20Action%20Object%20Reference :default "/Game/TrickPhotography/Programmers/Core/Inputs/IA_SkipCutscene.IA_SkipCutscene"))
  (if (Variables|Default|GetbIsAnimating)
    (Variables|Default|SetbIsAnimating false)
    (Default|CallOnAnimationFinished)
    (bind _asmain_player_controller (Utilities|Casting|CastToMainPlayerController (Pawn|GetController)))
    (Default|PossessMainCharacter _asmain_player_controller)))

(event EventActivate
  (bind _asmain_player_controller (Utilities|Casting|CastToMainPlayerController (Game|GetPlayerController 0)))
  (Default|PossessCutsceneCamera _asmain_player_controller self))

(event EventBeginPlay
  (Variables|Default|SetbIsAnimating false))

(event EventPossessed
  (params (NewController :type Controller%20Object%20Reference))
  (bind _audiosource (Variables|Default|GetAudioSource))
  (bind _jingle (Variables|Default|GetJingle))
  (Variables|Default|SetAnimationTime 0.0)
  (Variables|Default|SetbIsAnimating true)
  (Utilities|IsValid _jingle
    (:Is%20Valid
      (Audio|Components|Audio|SetSound _audiosource _jingle)
      (Audio|Components|Audio|Play _audiosource 0.0))))

(event EventUnpossessed
  (params (OldController :type Controller%20Object%20Reference))
  (Variables|Default|SetbIsAnimating false))

(event EventTick
  (params (DeltaSeconds :type Float%20%28single-precision%29))
  (bind _animationtime (Variables|Default|GetAnimationTime))
  (bind _track (Variables|Default|GetTrack))
  (bind _returnvalue (+ _animationtime DeltaSeconds))
  (bind _duration (Variables|/Script/Engine.SplineComponent|GetDuration _track))
  (bind _returnvalue_2 (>= _returnvalue _duration))
  (if (Variables|Default|GetbIsAnimating)
    (CallFunction|SetAnimationTime (Math|Float|SelectFloat _duration _returnvalue _returnvalue_2))
    (if _returnvalue_2
      (Variables|Default|SetbIsAnimating false)
      (Utilities|FlowControl|Delay (Variables|Default|GetWaitTimeAtEnd))
      (Default|CallOnAnimationFinished)
      (bind _asmain_player_controller (Utilities|Casting|CastToMainPlayerController (Pawn|GetController)))
      (Default|PossessMainCharacter _asmain_player_controller))))

(fn ConstructionScript)

(fn SetAnimationTime
  (params (NewTime :type Float%20%28double-precision%29))
  (bind _track (Variables|Default|GetTrack))
  (bind _duration (Variables|/Script/Engine.SplineComponent|GetDuration _track))
  (bind _output_get (Variables|Default|SetAnimationTime NewTime))
  (bind _returnvalue (CallFunction|GetCameraLocationbyTime (* _duration (Math|Curves|GetFloatValue (Variables|Default|GetAnimationCurve) (/ _output_get _duration)))))
  (Transformation|SetWorldTransform (Variables|Default|GetCamera) _returnvalue false true))

(fn GetCameraLocationbyTime
  (params (Time :type Float%20%28double-precision%29))
  (bind _track (Variables|Default|GetTrack))
  (bind _camera (Variables|Default|GetCamera))
  (bind _focuspoint (Variables|Default|GetFocusPoint))
  (bind _returnvalue (Spline|GetTransformatTime _track Time "World" false false))
  (bind _returnvalue_2 (Transformation|GetWorldTransform _camera))
  (bind (_location _rotation _scale) (Math|Transform|BreakTransform _returnvalue))
  (if (Variables|Default|GetStaticRotation)
    (return (Math|Transform|MakeTransform (.Location (Math|Transform|BreakTransform _returnvalue)) (.rotation _returnvalue_2) (.scale _returnvalue_2)))
    (else
      (Utilities|IsValid _focuspoint
        (:Is%20Valid
          (return (Math|Transform|MakeTransform _location (Math|Rotator|FindLookatRotation _location (.location (Transformation|GetActorTransform _focuspoint))) _scale)))
        (:Is%20Not%20Valid
          (return _returnvalue))))))