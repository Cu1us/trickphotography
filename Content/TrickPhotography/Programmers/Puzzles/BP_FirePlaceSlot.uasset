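; BP_FirePlaceSlot is an interactable puzzle fireplace that accepts a log and can then be lit.
; Interacting with a held BP_LogPickup activates it, and an overlapping pickup receives a slot reference.
; SetLogInFireplace reveals the hidden log, after which interacting without a log shows the point light and turns the decal from cold to hot color.
; Hover and interaction-type functions supply context prompts until the fire is lit.
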(event Custom|SetLogInFireplace
  (Rendering|SetVisibility (Variables|Default|GetLog) true false)
  (Collision|SetCollisionEnabled (Variables|Default|GetLog) "NoCollision")
  (Collision|SetCollisionEnabled (Variables|Default|GetBox) "QueryAndPhysics")
  (Variables|Default|SetbLogPlaced true))

(event EventInteractStart
  (params (HeldItem :type Pickupable%20Interface%20Interface) (bIsCammy :type Boolean) (HitComponent :type Primitive%20Component%20Object%20Reference))
  (bind _fireplacedecal (Variables|Default|GetFireplaceDecal))
  (if (not (Variables|Default|GetbLit))
    (Utilities|Casting|CastToBP_LogPickup HeldItem
      (:then
        (Class|PickupableInterface|Activate HeldItem (Transformation|GetWorldTransform (Variables|/Game/TrickPhotography/Programmers/Core/Player/BP_MainCharacter.BP_MainCharacter_C|GetFirstPersonCamera (Variables|/Game/TrickPhotography/Programmers/Core/Player/MainPlayerController.MainPlayerController_C|GetMainChar (Variables|Default|GetMainPlayerController)))) bIsCammy))
      (:CastFailed
        (if (Variables|Default|GetbLogPlaced)
          (Rendering|SetVisibility (Variables|Default|GetPointLight) true false)
          (Collision|SetCollisionEnabled (Variables|Default|GetLog) "NoCollision")
          (Variables|Default|SetbLit true)
          (Collision|SetCollisionEnabled (Variables|Default|GetBox) "QueryAndPhysics")
          (Utilities|IsValid _fireplacedecal
            (:Is%20Valid
              (Rendering|Components|Decal|SetDecalColor (Variables|/Script/trickphotography.FilterableDecalActor|GetDecal _fireplacedecal) (Variables|Default|GetHotColor)))))))))

(event Collision|EventActorBeginOverlap
  (params (OtherActor :type Actor%20Object%20Reference))
  (bind _asbp_log_pickup (Utilities|Casting|CastToBP_LogPickup OtherActor))
  (Default|LogCollidedwithFireplaceSlot _asbp_log_pickup self))

(event EventBeginPlay
  (bind _fireplacedecal (Variables|Default|GetFireplaceDecal))
  (|CallParentFunction)
  (Collision|SetCollisionEnabled (Variables|Default|GetLog) "NoCollision")
  (Rendering|SetVisibility (Variables|Default|GetLog) false false)
  (bind _asmain_player_controller (Utilities|Casting|CastToMainPlayerController (Game|GetPlayerController 0)))
  (Variables|Default|SetMainPlayerController _asmain_player_controller)
  (Utilities|IsValid _fireplacedecal
    (:Is%20Valid
      (Rendering|Components|Decal|SetDecalColor (Variables|/Script/trickphotography.FilterableDecalActor|GetDecal _fireplacedecal) (Variables|Default|GetColdColor)))))

(fn ConstructionScript)

(fn GetInteractionType
  (params (bIsCammy :type Boolean) (HitComponent :type Primitive%20Component%20Object%20Reference))
  (if (Variables|Default|GetbLit)
    (return "NewEnumerator5" "")
    (elif (== HitComponent (Variables|Default|GetLog))
      (return "NewEnumerator5" "Light Fire")
      (elif (== HitComponent (Variables|Default|GetBox))
        (return "NewEnumerator5" "Needs Firewood")
        (else
          (return "NewEnumerator5" ""))))))

(fn HoverOngoing
  (params (HeldItem :type Pickupable%20Interface%20Interface) (HitComponent :type Primitive%20Component%20Object%20Reference))
  (if (Variables|Default|GetbLit)
    (return false)
    (else
      (Utilities|Casting|CastToBP_LogPickup HeldItem
        (:then
          (return true))
        (:CastFailed
          (return true))))))

(fn HoverStart
  (params (HeldItem :type Pickupable%20Interface%20Interface) (HitComponent :type Primitive%20Component%20Object%20Reference) (bIsCammy :type Boolean))
  (if (Variables|Default|GetbLit)
    (return false)
    (else
      (bind _asmain_player_controller (Utilities|Casting|CastToMainPlayerController (Game|GetPlayerController 0)))
      (if (== HitComponent (Variables|Default|GetLog))
        (Variables|/Game/TrickPhotography/Programmers/Core/Player/BP_MainCharacter.BP_MainCharacter_C|SetInteractOverrideText (Variables|/Game/TrickPhotography/Programmers/Core/Player/MainPlayerController.MainPlayerController_C|GetMainChar _asmain_player_controller) "Light Fire 
")
        (else
          (Utilities|Casting|CastToBP_LogPickup HeldItem
            (:then
              (Variables|/Game/TrickPhotography/Programmers/Core/Player/BP_MainCharacter.BP_MainCharacter_C|SetInteractOverrideText (Variables|/Game/TrickPhotography/Programmers/Core/Player/MainPlayerController.MainPlayerController_C|GetMainChar _asmain_player_controller) "Place Log 
"))
            (:CastFailed
              (Variables|/Game/TrickPhotography/Programmers/Core/Player/BP_MainCharacter.BP_MainCharacter_C|SetInteractOverrideText (Variables|/Game/TrickPhotography/Programmers/Core/Player/MainPlayerController.MainPlayerController_C|GetMainChar _asmain_player_controller) "Need wood")))))
      (return true))))