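; BP_LatchLocker is an interactable puzzle locker whose lid opens once both the left and right latch handles are pulled.
; Interacting with a handle sets its pulled flag on the ABP_LatchLocker anim instance and disables that handle's collision, so each works only once.
; When both flags are set, short delays sequence the lid opening and then clear the pulled flags, while the lid stays open.
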(event EventInteractStart
  (params (HeldItem :type Pickupable%20Interface%20Interface) (bIsCammy :type Boolean) (HitComponent :type Primitive%20Component%20Object%20Reference))
  (bind _asabp_latch_locker (Utilities|Casting|CastToABP_LatchLocker (Components|SkeletalMesh|GetAnimInstance (Variables|Default|GetFilterSkeletalMesh))))
  (if (== HitComponent (Variables|Default|GetLeftHandle))
    (bind _output_get (Variables|/Game/TrickPhotography/Art/Puzzles/LatchLocker/ABP_LatchLocker.ABP_LatchLocker_C|SetLeftHandlePulled _asabp_latch_locker true))
    (Collision|SetCollisionEnabled (Variables|Default|GetLeftHandle) "NoCollision")
    (if (and _output_get (stale _output_get_2)) :!label _label
      (Utilities|FlowControl|Delay 0.4)
      (Variables|/Game/TrickPhotography/Art/Puzzles/LatchLocker/ABP_LatchLocker.ABP_LatchLocker_C|SetLidOpen _asabp_latch_locker true)
      (Utilities|FlowControl|Delay 1.0)
      (Variables|/Game/TrickPhotography/Art/Puzzles/LatchLocker/ABP_LatchLocker.ABP_LatchLocker_C|SetLeftHandlePulled _asabp_latch_locker false)
      (Variables|/Game/TrickPhotography/Art/Puzzles/LatchLocker/ABP_LatchLocker.ABP_LatchLocker_C|SetRightHandlePulled _asabp_latch_locker false))
    (elif (== HitComponent (Variables|Default|GetRightHandle))
      (bind _output_get_2 (Variables|/Game/TrickPhotography/Art/Puzzles/LatchLocker/ABP_LatchLocker.ABP_LatchLocker_C|SetRightHandlePulled _asabp_latch_locker true))
      (Collision|SetCollisionEnabled (Variables|Default|GetRightHandle) "NoCollision")
      (goto _label))))

(fn ConstructionScript)

(fn GetInteractionType
  (params (bIsCammy :type Boolean) (HitComponent :type Primitive%20Component%20Object%20Reference))
  (return "NewEnumerator0" ""))

(fn HoverOngoing
  (params (HeldItem :type Pickupable%20Interface%20Interface) (HitComponent :type Primitive%20Component%20Object%20Reference))
  (return false))

(fn HoverStart
  (params (HeldItem :type Pickupable%20Interface%20Interface) (HitComponent :type Primitive%20Component%20Object%20Reference) (bIsCammy :type Boolean))
  (return false))