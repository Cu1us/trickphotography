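; Interactable combination-vault puzzle with three wheels that start at random steps and must all reach the correct rotation to unlock.
; Hovering the knob shows a widget and enables dial input, turning the first wheel, whose pins recursively drag the next ones like a real safe.
; Wheel state is read from mesh yaw, and each move plays a tick and recolors that wheel's solution ring.
; Pulling the handle toggles the door through timelines if unlocked, otherwise plays a failed-handle animation.
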(event Custom|SetOpenState
  (params (Open :type Boolean))
  (if Open
    (bind _zrot (Timeline|DoorClose PlayFromStart)
      (:Update
        (Transformation|SetRelativeRotation (Variables|Default|GetHandle) (Math|Rotator|MakeRotator 0.0 0.0 (+ _zrot 1.8e+02)) false false))
      (:Finished
        (bind _openamount (Timeline|DoorOpenTimeline Play)
          (:Update
            (Transformation|SetRelativeRotation (Variables|Default|GetDoor) (Math|Rotator|MakeRotator -9e+01 0.0 _openamount) false false)))))
    (else
      (Timeline|DoorOpenTimeline Reverse))))

(event Input|EnhancedActionEvents|EnhancedInputActionIA_TurnDial
  (params (ActionValue :type Float%20%28double-precision%29) (ElapsedSeconds :type Float%20%28double-precision%29) (TriggeredSeconds :type Float%20%28double-precision%29) (InputAction :type Input%20Action%20Object%20Reference :default "/Game/TrickPhotography/Programmers/Core/Inputs/Vault/IA_TurnDial.IA_TurnDial"))
  (if (Variables|Default|GetbKnobSelected)
    (CallFunction|RotateWheel 0 (== ActionValue 1.0))
    (bind _unlocked (CallFunction|IsUnlocked))
    (if _unlocked
      _)))

(event EventBeginPlay
  (CallFunction|RandomizeDiscPositions)
  (bind _asmain_player_controller (Utilities|Casting|CastToMainPlayerController (Game|GetPlayerController 0)))
  (bind _output_get (Variables|Default|SetMainPlayerController _asmain_player_controller))
  (bind _returnvalue (UserInterface|CreateWidget "/Game/TrickPhotography/Programmers/Core/UI/WidgetVault.WidgetVault_C" _output_get))
  (bind _output_get_2 (Variables|Default|SetWidget _returnvalue))
  (UserInterface|Viewport|AddtoViewport _output_get_2 0)
  (Widget|SetVisibility _output_get_2 "Hidden"))

(event EventInteractEnd
  (params (bIsCammy :type Boolean) (HitComponent :type Primitive%20Component%20Object%20Reference)))

(event EventHoverEnd
  (params (HeldItem :type Pickupable%20Interface%20Interface) (bIsCammy :type Boolean))
  (if (not bIsCammy)
    (Variables|Default|SetbKnobSelected false)
    (Input|RemoveMappingContext (PlayerController|LocalPlayerSubsystems|GetEnhancedInputLocalPlayerSubsystem (Variables|Default|GetMainPlayerController)) "/Game/TrickPhotography/Programmers/Core/Inputs/Vault/IMC_Vault.IMC_Vault" "(bIgnoreAllPressedKeysUntilRelease=True,bForceImmediately=False,bNotifyUserSettings=False)")
    (Widget|SetVisibility (Variables|Default|GetWidget) "Hidden")))

(event EventInteractStart
  (params (HeldItem :type Pickupable%20Interface%20Interface) (bIsCammy :type Boolean) (HitComponent :type Primitive%20Component%20Object%20Reference))
  (if (== HitComponent (Variables|Default|GetHandle))
    (bind _unlocked (CallFunction|IsUnlocked))
    (if _unlocked
      (bind _isa (Utilities|FlowControl|FlipFlop)
        (:A
          _)
        (:B
          _))
      (CallFunction|SetOpenState _isa)
      (Development|PrintString "ok")
      (else
        (Development|PrintString "fail")
        (bind _zrot (Timeline|FailedHandle PlayFromStart)
          (:Update
            (Transformation|SetRelativeRotation (Variables|Default|GetHandle) (Math|Rotator|MakeRotator 0.0 0.0 (+ _zrot 1.8e+02)) false false)))))))

(fn ConstructionScript)

(fn RotateWheel
  (params (WheelIndex :type Integer) (Clockwise :type Boolean))
  (bind _returnvalue (+ WheelIndex 1))
  (bind _realpinrotation (Utilities|GetRealPinLocation WheelIndex)
    (:Then
      (bind _realpinrotation_2 (Utilities|GetRealPinLocation _returnvalue)
        (:Then
          (if (== (Math|Integer|SelectInt _realpinrotation_2 (Utilities|AddwithModulo _realpinrotation_2 1) Clockwise) _realpinrotation)
            (CallFunction|RotateWheel _returnvalue Clockwise)))
        (:Failed
          _))
      (bind _wheelrotation (Utilities|GetWheelRotation WheelIndex)
        (:then
          (Utilities|SetWheelRotation WheelIndex (Utilities|AddwithModulo _wheelrotation (Math|Integer|SelectInt 1 -1 Clockwise))))
        (:Failed
          _))
      (Utilities|PlayWheelTick WheelIndex))))

(fn RandomizeDiscPositions
  (for _index (range 0 (- (Class|SceneComponent|GetNumChildrenComponents (Variables|Default|GetDiscs)) 1))
    (Utilities|SetWheelRotation _index (Math|Random|RandomIntegerinRange 0 (- (Variables|Default|GetSteps) 1)))))

(fn EnableSolutionRing
  (params (Index :type Integer) (Enabled :type Boolean))
  (bind _small (Variables|Default|GetSmall))
  (bind _medium (Variables|Default|GetMedium))
  (bind _big (Variables|Default|GetBig))
  (bind _returnvalue (Utilities|Select :Index Index :Option%200 _small :Option%201 _medium :Option%202 _big))
  (Utilities|IsValid _returnvalue
    (:Is%20Valid
      (Rendering|Material|SetMaterial _returnvalue 0 (select Enabled (Variables|Default|GetSolutionRingCorrectMaterial) (Variables|Default|GetSolutionRingIncorrectMaterial))))))

(fn IsUnlocked
  (LocalVariables|SetbUnlocked true)
  (bind _array_index (Utilities|Array|ForEachLoopwithBreak (Utilities|GetDiscComponents) :!label _label)
    (:LoopBody
      (bind _wheelrotation (Utilities|GetWheelRotation _array_index)
        (:then
          (Development|PrintString (Utilities|String|ToString(Integer) (Math|Integer|Absolute(Integer) _wheelrotation)))
          (if (not (== (Math|Integer|Absolute(Integer) _wheelrotation) (Variables|Default|GetCorrectRotation)))
            (LocalVariables|SetbUnlocked false)
            (goto _label Break)))))
    (:Completed
      (return (LocalVariables|GetbUnlocked)))))

(fn GetInteractionType
  (params (bIsCammy :type Boolean) (HitComponent :type Primitive%20Component%20Object%20Reference))
  (if (== HitComponent (Variables|Default|GetHandle))
    (return "NewEnumerator5" "Pull Handle")
    (elif (== HitComponent (Variables|Default|GetKnob))
      (return "NewEnumerator5" "")
      (else
        (return "NewEnumerator0" "")))))

(fn HoverOngoing
  (params (HeldItem :type Pickupable%20Interface%20Interface) (HitComponent :type Primitive%20Component%20Object%20Reference))
  (bind _mainplayercontroller (Variables|Default|GetMainPlayerController))
  (bind _output_get (Variables|Default|SetbKnobSelected (== HitComponent (Variables|Default|GetKnob))))
  (if _output_get
    (Input|AddMappingContext (PlayerController|LocalPlayerSubsystems|GetEnhancedInputLocalPlayerSubsystem _mainplayercontroller) "/Game/TrickPhotography/Programmers/Core/Inputs/Vault/IMC_Vault.IMC_Vault" 2 "(bIgnoreAllPressedKeysUntilRelease=True,bForceImmediately=False,bNotifyUserSettings=False)")
    (Widget|SetVisibility (Variables|Default|GetWidget) "Visible")
    (Input|EnableInput _mainplayercontroller)
    (return true)
    (else
      (Variables|Default|SetbKnobSelected false)
      (Input|RemoveMappingContext (PlayerController|LocalPlayerSubsystems|GetEnhancedInputLocalPlayerSubsystem (Variables|Default|GetMainPlayerController)) "/Game/TrickPhotography/Programmers/Core/Inputs/Vault/IMC_Vault.IMC_Vault" "(bIgnoreAllPressedKeysUntilRelease=True,bForceImmediately=False,bNotifyUserSettings=False)")
      (Widget|SetVisibility (Variables|Default|GetWidget) "Hidden")
      (if (== HitComponent (Variables|Default|GetHandle))
        (return true)))))

(fn HoverStart
  (params (HeldItem :type Pickupable%20Interface%20Interface) (HitComponent :type Primitive%20Component%20Object%20Reference) (bIsCammy :type Boolean))
  (bind _mainplayercontroller (Variables|Default|GetMainPlayerController))
  (Development|PrintString (Utilities|GetDisplayName HitComponent))
  (bind _output_get (Variables|Default|SetbKnobSelected (== HitComponent (Variables|Default|GetKnob))))
  (if _output_get
    (Input|AddMappingContext (PlayerController|LocalPlayerSubsystems|GetEnhancedInputLocalPlayerSubsystem _mainplayercontroller) "/Game/TrickPhotography/Programmers/Core/Inputs/Vault/IMC_Vault.IMC_Vault" 2 "(bIgnoreAllPressedKeysUntilRelease=True,bForceImmediately=False,bNotifyUserSettings=False)")
    (Widget|SetVisibility (Variables|Default|GetWidget) "Visible")
    (Input|EnableInput _mainplayercontroller)
    (return true)
    (elif (== HitComponent (Variables|Default|GetHandle))
      (return true))))