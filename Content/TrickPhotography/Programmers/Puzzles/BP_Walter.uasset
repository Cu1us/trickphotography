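; BP_Walter is the final reveal puzzle object whose reveal from invisibility depends on linked machines and triggers the game's ending.
; Tick sums machine activation progress into custom primitive data on the Waltuh component.
; A reveal plays a scaled partial timeline until activation passes a threshold.
; Past it, a one-time full reveal timeline ends in TriggerEnding, while machines fire toward BeamTarget and a delayed sound sequence plays.
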(event EventOnInvisPhotoFinished
  (|CallParentFunction)
  (Rendering|SetVisibility (Variables|Default|GetWaltuh) true false))

(event EventOnInvisPhoto
  (|CallParentFunction))

(event EventBeginPlay
  (|CallParentFunction)
  (Rendering|SetVisibility (Variables|Default|GetWaltuh) true false))

(event EventOnRevealfromInvisibility
  (bind _waltuh (Variables|Default|GetWaltuh))
  (if (not (Variables|Default|GetbRevealed))
    (if (> (Variables|Default|GetMachinesActive) 2.8)
      (Utilities|FlowControl|Sequence
        (:then_0
          (Variables|Default|SetbRevealed true)
          (bind _revealamount (Timeline|RevealComplete PlayFromStart)
            (:Update
              (Rendering|Material|SetCustomPrimitiveDataFloat _waltuh 1 _revealamount))
            (:Finished
              (bind _asmain_player_controller (Utilities|Casting|CastToMainPlayerController (Game|GetPlayerController 0)))
              (Default|TriggerEnding _asmain_player_controller))))
        (:then_1
          (Utilities|FlowControl|Delay 0.25)
          (for _array_element (Variables|Default|GetMachines)
            (Default|TriggerReveal _array_element (Transformation|GetWorldLocation (Variables|Default|GetBeamTarget))))
          (Audio|Components|Audio|Play (Variables|Default|GetRevealMachineWhirr) 0.0)
          (Utilities|FlowControl|Delay 5.0)
          (Audio|Components|Audio|Play (Variables|Default|GetRevealShatter) 0.0)
          (Utilities|FlowControl|Delay 3.0)
          (Audio|Components|Audio|Play (Variables|Default|GetJumpLand) 0.0)
          (Utilities|FlowControl|Delay 1.0)
          (Audio|Components|Audio|Play (Variables|Default|GetCleanCoat) 0.0)
          (Utilities|FlowControl|Delay 4.0)
          (Audio|Components|Audio|Play (Variables|Default|GetFootstep) 0.0)))
      (else
        (bind _newtrack_0 (Timeline|RevealIncomplete PlayFromStart)
          (:Update
            (Rendering|Material|SetCustomPrimitiveDataFloat _waltuh 1 (* _newtrack_0 (+ (* (Variables|Default|GetMachinesActive) 0.15) 0.5)))))))))

(event EventTick
  (params (DeltaSeconds :type Float%20%28single-precision%29))
  (Variables|Default|SetMachinesActive 0.0)
  (for _array_element (Variables|Default|GetMachines)
    (bind _output_get (Variables|Default|SetMachinesActive (+ (stale _output_get) (Variables|/Game/TrickPhotography/Programmers/Puzzles/BP_StillLifeGenerator.BP_StillLifeGenerator_C|GetActivationProgress _array_element)))))
  (Rendering|Material|SetCustomPrimitiveDataFloat (Variables|Default|GetWaltuh) 0 _output_get))

(fn ConstructionScript)