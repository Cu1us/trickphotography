(event Custom|TalkToDoor
  (bind _uiref (Variables|Default|GetUIRef))
  (if (Variables|Default|GetbFridgeSaved)
    (Default|SetDialogText _uiref "Thanks again for saving me <3" 1e+01)
    (else
      (Default|SetDialogText _uiref "I'm overheating, please clear the blockage in my cooling vents!" 1e+01))))

(event EventBeginPlay
  (Variables|Default|SetRelative%20Rotation%20Z%20%28Yaw%29 (.yaw (Transformation|GetWorldRotation (Variables|Default|GetDoor))))
  (bind _asmain_player_controller (Utilities|Casting|CastToMainPlayerController (Game|GetPlayerController 0)))
  (Variables|Default|SetUIRef (Variables|/Game/TrickPhotography/Programmers/Core/Player/MainPlayerController.MainPlayerController_C|GetUIRef _asmain_player_controller)))

(event EventTick
  (params (DeltaSeconds :type Float%20%28single-precision%29))
  (if (Variables|Default|GetbFridgeSaved)
    (Transformation|AddRelativeRotation (Variables|Default|GetFan) (Math|Rotator|MakeRotator (* (Variables|Default|GetFanSpeed) DeltaSeconds) 0.0 0.0) false false)))

(event EventActivate
  (bind _door (Variables|Default|GetDoor))
  (bind _returnvalue (Transformation|GetWorldRotation _door))
  (bind _rotation (Timeline|FridgeOpen Play)
    (:Update
      (Transformation|SetWorldRotation (Variables|Default|GetDoor) (Math|Rotator|MakeRotator (.roll _returnvalue) (.pitch _returnvalue) (+ _rotation (Variables|Default|GetRelative%20Rotation%20Z%20%28Yaw%29))) false false))
    (:Finished
      (Variables|Default|SetbFridgeSaved true)
      (Default|SetDialogText (Variables|Default|GetUIRef) "Thanks for cooling me down, remember to grab the UV filter from my belly." 1e+01))))

(fn ConstructionScript)