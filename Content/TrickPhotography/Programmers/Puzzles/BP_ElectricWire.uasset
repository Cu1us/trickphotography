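; BP_ElectricWire is a puzzle wire actor whose appearance in thermal photos reflects whether it is activated.
; Activate and Deactivate only toggle the Activated flag, without refreshing the visuals.
; On OnThermalPhoto, ThermalVisibility decides the response: Visible applies the activated or default thermal material based on that flag, while Hidden hides the actor in game.
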(event EventBeginPlay
  (|CallParentFunction) ; This node is disabled and will not be called.\nDrag off pins to build functionality.
)

(event EventOnThermalPhoto
  (switch Utilities|FlowControl|Switch|SwitchonFilterVisibility (Variables|Default|GetThermalVisibility)
    (:Visible
      (CallFunction|SetMaterial (select (Variables|Default|GetbActivated) (Variables|Cable|Thermal|GetThermalMaterialActivated) (Variables|Default|GetThermalMaterial))))
    (:Hidden
      (Rendering|SetActorHiddenInGame true))))

(event EventActivate
  (Variables|Default|SetbActivated true))

(event EventDeactivate
  (Variables|Default|SetbActivated false))

(fn ConstructionScript
  (|CallParentFunction))