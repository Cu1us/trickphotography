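; A puzzle pot that Cammy's character knocks over by entering its trigger sphere, spawning a configurable object when it shatters.
; The first overlap enables physics on the geometry collection and applies a directional impulse at a set point.
; Its first Chaos break spawns the object there, plays sound and camera shake, and fires OnBreak.
; The construction script applies model, sound and collider settings, and previews the impulse with an arrow.
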(event OnComponentBeginOverlap(Collider)
  (params (OverlappedComponent :type Primitive%20Component%20Object%20Reference) (OtherActor :type Actor%20Object%20Reference) (OtherComp :type Primitive%20Component%20Object%20Reference) (OtherBodyIndex :type Integer) (bFromSweep :type Boolean) (SweepResult :type Hit%20Result%20Structure%20%28by%20ref%29))
  (bind _pot (Variables|Default|GetPot))
  (bind _returnvalue (Transformation|GetWorldTransform _pot))
  (if (not (Variables|Knockable|GetbActivated))
    (Utilities|Casting|CastToBP_CammyCharacter OtherActor)
    (Variables|Knockable|SetbActivated true)
    (Physics|SetSimulatePhysics _pot true)
    (Physics|AddImpulseatLocation _pot (* (Math|Vector|GetForwardVector (Math|Transform|TransformRotation _returnvalue (Variables|Knockable|Launching|GetInitialVelocityDir))) (Variables|Knockable|Launching|GetInitialVelocity) (Math|Float|MakeLiteralFloat 7.5e+03)) (Math|Transform|TransformLocation _returnvalue (Variables|Knockable|Launching|GetInitialVelocityLocation)) "None")))

(event OnChaosBreakEvent(Pot)
  (params (BreakEvent :type Chaos%20Break%20Event%20Structure%20%28by%20ref%29))
  (if (not (Variables|Knockable|Destruction|GetbBroken))
    (Variables|Knockable|Destruction|SetbBroken true)
    (Development|PrintString "it broke, wahoo")
    (Game|SpawnActorfromClass (Variables|Knockable|Destruction|GetObejctToSpawn) (Math|Transform|MakeTransform (.location BreakEvent) "0, 0, 0" "1.000000,1.000000,1.000000") "AlwaysSpawn" "MultiplyWithRoot" 0 0)
    (Audio|Components|Audio|Play (Variables|Default|GetBreakSoundSource) 0.2)
    (CameraShakes|StartCameraShake (Variables|Default|GetCameraShakeSource) (Variables|Knockable|Destruction|GetCameraShake) (Variables|Knockable|Destruction|GetCameraShakeMultiplier) "CameraLocal" "0, 0, 0")
    (Default|CallOnBreak)))

(event EventBeginPlay
  (Physics|SetSimulatePhysics (Variables|Default|GetPot) false))

(fn ConstructionScript
  (bind _arrow (Variables|Default|GetArrow))
  (bind _breaksound (Variables|Knockable|Destruction|GetBreakSound))
  (Transformation|SetRelativeLocationAndRotation _arrow (Variables|Knockable|Launching|GetInitialVelocityLocation) (Variables|Knockable|Launching|GetInitialVelocityDir) false false)
  (Variables|/Script/Engine.ArrowComponent|SetArrowLength _arrow (* (Math|Float|Sqrt (Variables|Knockable|Launching|GetInitialVelocity)) 33.0))
  (Transformation|SetRelativeLocation (Variables|Default|GetPot) (Variables|Knockable|GetHitboxOffset) false false)
  (Components|Sphere|SetSphereRadius (Variables|Default|GetCollider) (Variables|Knockable|GetColliderRadius) false)
  (Utilities|FlowControl|Sequence
    (:then_0
      (Utilities|IsValid _breaksound
        (:Is%20Valid
          (Audio|Components|Audio|SetSound (Variables|Default|GetBreakSoundSource) _breaksound))))
    (:then_1
      (Utilities|IsValid (Variables|Knockable|GetModel)
        (:Is%20Valid
          (Class|GeometryCollectionComponent|SetRestCollection (Variables|Default|GetPot) (Variables|Knockable|GetModel) false))))))