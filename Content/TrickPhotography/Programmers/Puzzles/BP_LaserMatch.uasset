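; Laser puzzle match actor that heats up under a laser, ignites, burns and then destroys itself.
; LightBuildup calls raise a clamped temperature and hold a laser-active flag through a retriggerable delay; without them, the heat collapses to near zero.
; Tick feeds heat into smoke intensity until the ignition threshold, then swaps to the burned mesh with flame and sound.
; A timeline then drives fire intensity and actor scale until destruction.
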(event Custom|LightBuildup
  (Variables|Default|SetbLaserActive true)
  (Variables|Default|SetbTemp (Math|Float|Clamp(Float) (+ 0.05 (Variables|Default|GetbTemp)) 0.0 1.5))
  (Utilities|FlowControl|RetriggerableDelay 0.2)
  (Variables|Default|SetbLaserActive false))

(event EventTick
  (params (DeltaSeconds :type Float%20%28single-precision%29))
  (if (Variables|Default|GetbLit)
    (Niagara|SetNiagaraVariable(Float) (Variables|Default|GetSmoke) "FlameIntensity" (stale _newtrack_0))
    (else
      (Niagara|SetNiagaraVariable(Float) (Variables|Default|GetSmoke) "FlameIntensity" (Variables|Default|GetbTemp))
      (if (Variables|Default|GetbLaserActive)
        (Variables|Default|SetbLit (>= (stale _output_get) 1.3))
        (else
          (bind _output_get (Variables|Default|SetbTemp (Math|Float|Clamp(Float) (- 0.05 (Variables|Default|GetbTemp)) 0.0 1.5)))))
      (if (Variables|Default|GetbLit)
        (Rendering|SetVisibility (Variables|Default|GetFlame) true false)
        (Components|Activation|Activate (Variables|Default|GetMatch_Ignite) false)
        (Audio|PlaySoundatLocation "/Game/TrickPhotography/Audio/Metasounds/MS_Match.MS_Match" (Transformation|GetActorLocation) "0, 0, 0" 1.0 1.0 0.0 0 0 0 0)
        (Rendering|SetVisibility (Variables|Default|GetBurnedMatch) true false)
        (Rendering|SetVisibility (Variables|Default|GetMatch) false false)
        (bind _newtrack_0 (Timeline|FireTimeline Play)
          (:Update
            (Niagara|SetNiagaraVariable(Float) (Variables|Default|GetFlame) "FlameIntensity" (* _newtrack_0 1.6))
            (Transformation|SetWorldScale3D (Variables|Default|GetSceneRoot) (Math|Conversions|ToVector(Float) _newtrack_0)))
          (:Finished
            (Actor|DestroyActor)))))))

(fn ConstructionScript)