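; Interactable teleport point that, when usable, moves the Cammy character along a spline or instantly to a target point, and highlights when Cammy hovers it.
; In spline mode, InteractStart flags Cammy as teleporting and enables Tick, which advances progress over the spline duration, remapped by a float curve.
; Tick faces Cammy along the tangent with scaled vertical tilt, then clears the flag and disables itself at the end.
; An older timeline-driven movement remains unconnected.
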(event EventHoverEnd
  (params (HeldItem :type Pickupable%20Interface%20Interface) (bIsCammy :type Boolean))
  (if bIsCammy
    (Class|FilterActor|SetPPMHighlight "None")))

(event EventTick
  (params (DeltaSeconds :type Float%20%28single-precision%29))
  (bind _spline (Variables|Default|GetSpline))
  (bind _duration (Variables|/Script/Engine.SplineComponent|GetDuration _spline))
  (if (< (Variables|Spline|GetSplineProgress) 0.0)
    (Actor|Tick|SetActorTickEnabled false)
    (else
      (bind _output_get (Variables|Spline|SetSplineProgress (Math|Float|Clamp(Float) (+ DeltaSeconds (stale _output_get)) 0.0 _duration)))
      (Transformation|SetActorLocationAndRotation (Variables|Default|GetTeleportingActor) (Spline|GetLocationatTime _spline (* (Math|Curves|GetFloatValue (Variables|Spline|GetSplineCurve) (/ _output_get _duration)) _duration) "World" false) (Math|Rotator|FindLookatRotation (Math|Vector|MakeVector 0.0 0.0 0.0) (Math|Vector|MakeVector (.x (Class|SplineComponent|GetTangentatTime _spline (* (Math|Curves|GetFloatValue (Variables|Spline|GetSplineCurve) (/ _output_get _duration)) _duration) "World" false)) (.y (Class|SplineComponent|GetTangentatTime _spline (* (Math|Curves|GetFloatValue (Variables|Spline|GetSplineCurve) (/ _output_get _duration)) _duration) "World" false)) (* (.z (Class|SplineComponent|GetTangentatTime _spline (* (Math|Curves|GetFloatValue (Variables|Spline|GetSplineCurve) (/ _output_get _duration)) _duration) "World" false)) (Variables|Spline|GetSplineMaxTiltMultiplier)))) false true)
      (if (== _duration (Math|Float|Clamp(Float) (+ DeltaSeconds _output_get) 0.0 _duration))
        (Variables|Spline|SetSplineProgress -1.0)
        (Default|SetTeleporting (Variables|Default|GetTeleportingActor) false)
        (Actor|Tick|SetActorTickEnabled false)))))

(event EventInteractStart
  (params (HeldItem :type Pickupable%20Interface%20Interface) (bIsCammy :type Boolean) (HitComponent :type Primitive%20Component%20Object%20Reference))
  (if (and bIsCammy (Variables|Interaction|GetbUsable))
    (bind _asmain_player_controller (Utilities|Casting|CastToMainPlayerController (Game|GetPlayerController 0)))
    (bind _output_get (Variables|Default|SetTeleportingActor (Variables|/Game/TrickPhotography/Programmers/Core/Player/MainPlayerController.MainPlayerController_C|GetCammyChar _asmain_player_controller)))
    (if (not (Variables|/Game/TrickPhotography/Programmers/Core/Player/BP_CammyCharacter.BP_CammyCharacter_C|GetbTeleporting _output_get))
      (if (< (Variables|Spline|GetSplineProgress) 0.0)
        (if (Variables|Spline|GetbUseSplineMovement)
          (Default|SetTeleporting (Variables|Default|GetTeleportingActor) true)
          (Variables|Spline|SetSplineProgress 0.0)
          (Actor|Tick|SetActorTickEnabled true)
          (else
            (Transformation|SetActorLocation (Variables|Default|GetTeleportingActor) (Transformation|GetActorLocation (Variables|Interaction|GetTargetPointIfNoSpline)) false true)))))))

(fn ConstructionScript
  (Variables|/Script/Engine.SplineComponent|SetDuration (Variables|Default|GetSpline) (Variables|Spline|GetSplineDuration)))

(fn GetInteractionType
  (params (bIsCammy :type Boolean) (HitComponent :type Primitive%20Component%20Object%20Reference))
  (if bIsCammy
    (return "NewEnumerator5" (Variables|Default|GetTooltip))
    (else
      (return "NewEnumerator5" ""))))

(fn HoverOngoing
  (params (HeldItem :type Pickupable%20Interface%20Interface) (HitComponent :type Primitive%20Component%20Object%20Reference))
  (return false))

(fn HoverStart
  (params (HeldItem :type Pickupable%20Interface%20Interface) (HitComponent :type Primitive%20Component%20Object%20Reference) (bIsCammy :type Boolean))
  (if bIsCammy
    (Class|FilterActor|SetPPMHighlight "HighlightHint")
    (return false)))