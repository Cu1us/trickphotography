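; BP_InvisRevealMesh is a temporary effect actor that plays an invisibility reveal on a given mesh for a target actor.
; A timeline drives Progress on a dynamic M_InvisReveal material, then unhides the target, activates Niagara and switches the material's Stage.
; It nudges the mesh toward the camera to avoid z-fighting.
; A second timeline drives Progress again, then the actor destroys itself after a short delay.
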(event EventBeginPlay
  (bind _staticmesh (Variables|Default|GetStaticMesh))
  (bind _staticmesh_2 (Variables|Default|GetStaticMesh))
  (bind _returnvalue (Transformation|GetWorldTransform _staticmesh_2))
  (Components|StaticMesh|SetStaticMesh _staticmesh (Variables|Default|GetMesh))
  (bind _returnvalue_2 (Rendering|Material|CreateDynamicMaterialInstance _staticmesh 0 "/Game/TrickPhotography/Art/Enviroment/Enviroment_Shaders/M_InvisReveal.M_InvisReveal" "None" :!class /Script/Engine.PrimitiveComponent))
  (Variables|Default|SetMaterialInstance _returnvalue_2)
  (bind _newtrack_0 (Timeline|Timeline Play)
    (:Update
      (Rendering|Material|SetScalarParameterValue (Variables|Default|GetMaterialInstance) "Progress" _newtrack_0 :!class /Script/Engine.MaterialInstanceDynamic))
    (:Finished
      (Rendering|SetActorHiddenInGame (Variables|Default|GetTarget) false)
      (Components|Activation|Activate (Variables|Default|GetNS_InvisReveal) false)
      (Rendering|Material|SetScalarParameterValue (Variables|Default|GetMaterialInstance) "Stage" 1.0 :!class /Script/Engine.MaterialInstanceDynamic)
      ;[0.15 0.15 0.15 0.5] Move object closer to camera + scale it up to avoid z fighting
      (Transformation|SetWorldTransform _staticmesh_2 (Math|Transform|MakeTransform (+ (.location _returnvalue) (* (Math|Vector|Normalize (- (Camera|GetCameraLocation (Game|GetPlayerCameraManager 0)) (.location _returnvalue))) (Math|Float|MakeLiteralFloat 1.0))) (.rotation _returnvalue) (* (.scale _returnvalue) (Math|Float|MakeLiteralFloat 1.0))) false true)
      (bind _newtrack_0_2 (Timeline|FinalStage Play)
        (:Update
          (Rendering|Material|SetScalarParameterValue (Variables|Default|GetMaterialInstance) "Progress" _newtrack_0_2 :!class /Script/Engine.MaterialInstanceDynamic))
        (:Finished
          (Utilities|FlowControl|Delay 4.0)
          (Actor|DestroyActor))))))

(fn ConstructionScript)