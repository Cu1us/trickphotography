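; BP_LaserPointer is a puzzle laser that traces a line forward from its root every tick while enabled.
; The trace endpoints position the Beam effect through its Start and End variables.
; Hitting a BP_LaserMatch calls its light buildup each tick.
; Hitting a BP_BurnablePainting burns it at the impact point, disables the laser and hides the beam after a short delay.
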(event EventTick
  (params (DeltaSeconds :type Float%20%28single-precision%29))
  (bind _defaultsceneroot (Variables|Default|GetDefaultSceneRoot))
  (bind _returnvalue (Transformation|GetWorldTransform _defaultsceneroot))
  (if (Variables|Default|GetbEnabled)
    (bind _outhit (Collision|LineTraceByChannel (.location _returnvalue) (+ (.location _returnvalue) (* (Math|Vector|GetForwardVector (.rotation _returnvalue)) (Math|Float|MakeLiteralFloat 3e+03))) "TraceTypeQuery4" true 0 "None" true "(R=0.000000,G=1.000000,B=0.404463,A=1.000000)" "(R=0.316096,G=0.000000,B=1.000000,A=1.000000)" 0.1))
    (CallFunction|SetLaserPoints (.TraceStart (Collision|BreakHitResult _outhit)) (.ImpactPoint (Collision|BreakHitResult _outhit)))
    (bind _asbp_laser_match (Utilities|Casting|CastToBP_LaserMatch (.HitActor (Collision|BreakHitResult _outhit)))
      (:then
        (Default|LightBuildup _asbp_laser_match))
      (:CastFailed
        (bind _asbp_burnable_painting (Utilities|Casting|CastToBP_BurnablePainting (.HitActor (Collision|BreakHitResult _outhit))))
        (Default|Burn _asbp_burnable_painting (.ImpactPoint (Collision|BreakHitResult _outhit)))
        (Variables|Default|SetbEnabled false)
        (Utilities|FlowControl|Delay 3.5)
        (Rendering|SetVisibility (Variables|Default|GetBeam) false false)))))

(fn ConstructionScript)

(fn SetLaserPoints
  (params (Start :type Vector) (End :type Vector))
  (bind _beam (Variables|Default|GetBeam))
  (Class|NiagaraComponent|SetVariablePosition _beam "Start" Start)
  (Class|NiagaraComponent|SetVariablePosition _beam "End" End))