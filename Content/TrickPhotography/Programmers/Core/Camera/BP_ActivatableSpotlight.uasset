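; BP_ActivatableSpotlight is a spotlight toggled by an activation source, with separate visibility for normal view and thermal, UV and X-ray photos.
; Activation events, optionally inverted, set one visibility flag, while photo events set a filter flag from per-mode settings, restoring the player setting when a photo finishes.
; The light shows only when both flags are true.
; The construction script can keep it visible in the editor.
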(event EventBeginPlay
  (bind _activationsource (Variables|Activation|GetActivationSource))
  (EventDispatchers|BindEventtoOnActivated _activationsource (delegate EventActivate))
  (EventDispatchers|BindEventtoOnDeactivated _activationsource (delegate EventDeactivate))
  (Variables|Default|SetbFilterVisibility (Variables|FilterInteraction|GetbVisibleByPlayer))
  (Variables|Default|SetbActivationVisibility (Variables|Activation|GetbIsInverse))
  (Utilities|UpdateVisibility))

(event EventOnAnyPhotoFinished
  (Variables|Default|SetbFilterVisibility (Variables|FilterInteraction|GetbVisibleByPlayer))
  (Utilities|UpdateVisibility))

(event EventDeactivate
  (Variables|Default|SetbActivationVisibility (Variables|Activation|GetbIsInverse))
  (Utilities|UpdateVisibility))

(event EventActivate
  (Variables|Default|SetbActivationVisibility (not (Variables|Activation|GetbIsInverse)))
  (Utilities|UpdateVisibility))

(event EventOnThermalPhoto
  (Variables|Default|SetbFilterVisibility (Variables|FilterInteraction|GetbVisibleInThermal))
  (Utilities|UpdateVisibility))

(event EventOnUVPhoto
  (Variables|Default|SetbFilterVisibility (Variables|FilterInteraction|GetbVisibleInUV))
  (Utilities|UpdateVisibility))

(event EventOnXrayPhoto
  (Variables|Default|SetbFilterVisibility (Variables|FilterInteraction|GetbVisibleInXray))
  (Utilities|UpdateVisibility))

(fn ConstructionScript
  (Rendering|SetVisibility (Variables|Default|GetSpotLightComponent) (or (Variables|Default|GetbAlwaysShowInEditor) (Variables|FilterInteraction|GetbVisibleByPlayer)) false))