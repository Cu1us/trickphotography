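; BP_Photograph is a photo item that characters can pick up, hold and pin to walls, with hover highlighting.
; SetImage creates a dynamic material by filter type, using an invisible variant for one filter, then sets texture and random seed.
; A timeline curve drives the image opacity to fade the photo in.
; Wall attachment toggles physics and pin visibility, while pickup swaps the mesh depending on whether Cammy holds it.
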(event Custom|FadeIn
  (bind _photofadeincurve (Timeline|PhotoFadeTimeline Play)
    (:Update
      (CallFunction|SetFadeAmount _photofadeincurve))))

(event Custom|SetAttachedToWall
  (params (bAttachToWall :type Boolean))
  (bind _output_get (Variables|Default|SetbIsAttachedToWall bAttachToWall))
  (Physics|SetSimulatePhysics (Variables|Default|GetPhotograph) (not _output_get))
  (Rendering|SetVisibility (Variables|Default|GetPin) _output_get false)
  (if _output_get
    (Audio|PlaySoundatLocation "/Game/TrickPhotography/Audio/Metasounds/MS_Pin.MS_Pin" (Transformation|GetActorLocation) "0, 0, 0" 1.0 1.0 0.0 0 0 0 0)))

(event EventOnPickup
  (params (isCammy :type Boolean))
  (|CallParentFunction isCammy)
  (if isCammy
    (if (Variables|Default|GetbIsAttachedToWall)
      _
      (else
        (Components|StaticMesh|SetStaticMesh (Variables|Default|GetPhotograph) (Variables|Default|GetHeldByCammyMesh))))
    (else
      (Components|StaticMesh|SetStaticMesh (Variables|Default|GetPhotograph) (Variables|Default|GetDefaultMesh))))
  (Rendering|SetVisibility (Variables|Default|GetPin) (Variables|Default|GetbIsAttachedToWall) false)
  (Audio|PlaySoundatLocation "/Game/TrickPhotography/Audio/Metasounds/MS_Pickup_Photo.MS_Pickup_Photo" (Transformation|GetActorLocation) "0, 0, 0" 1.0 1.0 0.0 0 0 0 0))

(event EventHoverEnd
  (params (HeldItem :type Pickupable%20Interface%20Interface) (bIsCammy :type Boolean))
  (Class|FilterActor|SetPPMHighlight "None"))

(fn ConstructionScript)

(fn SetImage
  (params (Image :type Texture%20Object%20Reference) (FilterTypeIn :type FilterType%20Enum :default "NewEnumerator0"))
  (bind _photograph (Variables|Default|GetPhotograph))
  (Utilities|IsValid (Variables|Default|GetPhotoMaterialInstance)
    (:Is%20Valid
      _)
    (:Is%20Not%20Valid
      (if (Utilities|Enum|Equal(Enum) FilterTypeIn "NewEnumerator5")
        (bind _returnvalue (Rendering|Material|CreateDynamicMaterialInstance _photograph 1 "/Game/TrickPhotography/Art/Enviroment/Materials_MeshSpecific/Photograph/M_Photograph_Invis.M_Photograph_Invis" "None" :!class /Script/Engine.PrimitiveComponent))
        (Variables|Default|SetPhotoMaterialInstance _returnvalue)
        (else
          (bind _returnvalue_2 (Rendering|Material|CreateDynamicMaterialInstance _photograph 1 "/Game/TrickPhotography/Art/Enviroment/Materials_MeshSpecific/Photograph/M_Photograph_Photo.M_Photograph_Photo" "None" :!class /Script/Engine.PrimitiveComponent))
          (Variables|Default|SetPhotoMaterialInstance _returnvalue_2)))))
  (Rendering|Material|SetTextureParameterValue (Variables|Default|GetPhotoMaterialInstance) "Image" Image)
  (Rendering|Material|SetScalarParameterValue (Variables|Default|GetPhotoMaterialInstance) "RandomSeed" (Math|Random|RandomFloat) :!class /Script/Engine.MaterialInstanceDynamic)
  (Variables|Default|SetFilterType FilterTypeIn))

(fn SetFadeAmount
  (params (ImageOpacity :type Float%20%28double-precision%29))
  (bind _photomaterialinstance (Variables|Default|GetPhotoMaterialInstance))
  (Utilities|IsValid _photomaterialinstance
    (:Is%20Valid
      (Rendering|Material|SetScalarParameterValue _photomaterialinstance "Opacity" (Math|Float|Clamp(Float) ImageOpacity) :!class /Script/Engine.MaterialInstanceDynamic))))

(fn GetCustomTransforms
  (return (Variables|Default|GetHeldTransform) (Variables|Default|GetLook%20at%20Transform) false false))

(fn GetInteractionType
  (params (bIsCammy :type Boolean) (HitComponent :type Primitive%20Component%20Object%20Reference))
  (return "NewEnumerator0" ""))

(fn HoverOngoing
  (params (HeldItem :type Pickupable%20Interface%20Interface) (HitComponent :type Primitive%20Component%20Object%20Reference))
  (return false))

(fn HoverStart
  (params (HeldItem :type Pickupable%20Interface%20Interface) (HitComponent :type Primitive%20Component%20Object%20Reference) (bIsCammy :type Boolean))
  (Class|FilterActor|SetPPMHighlight "HighlightPickup")
  (return false))