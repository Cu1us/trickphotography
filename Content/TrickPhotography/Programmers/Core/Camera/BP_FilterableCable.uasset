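; A cable actor that changes its look or disappears when thermal, UV or X-ray trick photos are taken.
; The construction script rebuilds it by tiling spline mesh segments along the spline, spaced by the mesh's X length with clamped tangents.
; Each photo start event checks that filter's visibility setting to swap all segments to the filter material or hide the actor.
; The matching finish event restores the default material or unhides it.
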(event EventBeginPlay
  (CallFunction|SetMaterial (Variables|Cable|GetDefaultMaterial)))

(event EventOnThermalPhoto
  ;[0.15 0.15 0.15 0.5] Photo Started
  (switch Utilities|FlowControl|Switch|SwitchonFilterVisibility (Variables|Cable|Thermal|GetThermalVisibility)
    (:Visible
      (CallFunction|SetMaterial (Variables|Cable|Thermal|GetThermalMaterial)))
    (:Hidden
      (Rendering|SetActorHiddenInGame true))))

(event EventOnUVPhoto
  ;[0.15 0.15 0.15 0.5] Photo Started
  (switch Utilities|FlowControl|Switch|SwitchonFilterVisibility (Variables|Cable|UV|GetUVVisibility)
    (:Visible
      (CallFunction|SetMaterial (Variables|Cable|UV|GetUVMaterial)))
    (:Hidden
      (Rendering|SetActorHiddenInGame true))))

(event EventOnXrayPhoto
  ;[0.15 0.15 0.15 0.5] Photo Started
  (switch Utilities|FlowControl|Switch|SwitchonFilterVisibility (Variables|Cable|Xray|GetXrayVisibility)
    (:Visible
      (CallFunction|SetMaterial (Variables|Cable|Xray|GetXrayMaterial)))
    (:Hidden
      (Rendering|SetActorHiddenInGame true))))

(event EventOnThermalPhotoFinished
  ;[0.15 0.15 0.15 0.5] Photo Finished
  (switch Utilities|FlowControl|Switch|SwitchonFilterVisibility (Variables|Cable|Thermal|GetThermalVisibility)
    (:Visible
      (CallFunction|SetMaterial (Variables|Cable|GetDefaultMaterial)))
    (:Hidden
      (Rendering|SetActorHiddenInGame false))))

(event EventOnUVPhotoFinished
  ;[0.15 0.15 0.15 0.5] Photo Finished
  (switch Utilities|FlowControl|Switch|SwitchonFilterVisibility (Variables|Cable|UV|GetUVVisibility)
    (:Visible
      (CallFunction|SetMaterial (Variables|Cable|GetDefaultMaterial)))
    (:Hidden
      (Rendering|SetActorHiddenInGame false))))

(event EventOnXrayPhotoFinished
  ;[0.15 0.15 0.15 0.5] Photo Finished
  (switch Utilities|FlowControl|Switch|SwitchonFilterVisibility (Variables|Cable|Xray|GetXrayVisibility)
    (:Visible
      (CallFunction|SetMaterial (Variables|Cable|GetDefaultMaterial)))
    (:Hidden
      (Rendering|SetActorHiddenInGame false))))

(fn ConstructionScript
  (CallFunction|Rebuild))

(fn Rebuild
  (bind _splinemesh (Variables|Cable|GetSplineMesh))
  (bind _spline (Variables|Default|GetSpline))
  (bind _spline_2 (Variables|Default|GetSpline))
  (bind _returnvalue (StaticMesh|GetBoundingBox _splinemesh))
  (Utilities|Array|Clear (Variables|Default|GetSegmentMeshes))
  (bind _output_get (LocalVariables|SetMeshLengthX (.x (- (.max _returnvalue) (.min _returnvalue)))))
  (for _index (range 0 (Math|Float|Floor (/ (Spline|GetSplineLength (Variables|Default|GetSpline)) _output_get)))
    (bind _returnvalue_2 (AddComponent|AddSplineMeshComponent false))
    (Components|StaticMesh|SetStaticMesh _returnvalue_2 (Variables|Cable|GetSplineMesh))
    (SplineMesh|SetStartandEnd _returnvalue_2 (Spline|GetLocationatDistanceAlongSpline _spline_2 (* _index (LocalVariables|GetMeshLengthX)) "Local") (Math|Vector|ClampVectorSize (Spline|GetTangentatDistanceAlongSpline _spline_2 (* _index (LocalVariables|GetMeshLengthX)) "Local") 0.0 1.0) (Spline|GetLocationatDistanceAlongSpline _spline (+ (* _index (LocalVariables|GetMeshLengthX)) (LocalVariables|GetMeshLengthX)) "Local") (Math|Vector|ClampVectorSize (Spline|GetTangentatDistanceAlongSpline _spline (+ (* _index (LocalVariables|GetMeshLengthX)) (LocalVariables|GetMeshLengthX)) "Local") 0.0 1.0) true :!class /Script/Engine.SplineMeshComponent)
    (Utilities|Array|AddUnique (Variables|Default|GetSegmentMeshes) _returnvalue_2)))

(fn SetMaterial
  (params (Material :type Material%20Interface%20Object%20Reference))
  (for _array_element (Variables|Default|GetSegmentMeshes)
    (Rendering|Material|SetMaterial _array_element 0 Material)))