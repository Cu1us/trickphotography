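; BP_InvisiDoor is a door concealed by a wall that appears and swings open when revealed from invisibility.
; The reveal extends the parent event: it hides the wall and its collision, then next tick switches Visibility-channel blocking from the frame to the door.
; After a short delay, a timeline rotates the door's scene component open, guarded by an Opened flag.
; Interaction queries give the door its own type, while hover handlers return false.
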(event Custom|OpenDoor
  (if (not (Variables|Default|GetbOpened))
    (bind _doorrot (Timeline|Timeline Play)
      (:Update
        (Transformation|SetRelativeRotation (Variables|Default|GetScene) (Math|Rotator|MakeRotator 0.0 0.0 _doorrot) false false)
        (Variables|Default|SetbOpened true)))))

(event EventBeginPlay)

(event Collision|EventActorBeginOverlap
  (params (OtherActor :type Actor%20Object%20Reference)))

(event EventTick
  (params (DeltaSeconds :type Float%20%28single-precision%29)))

(event EventOnRevealfromInvisibility
  (|CallParentFunction)
  (Rendering|SetVisibility (Variables|Default|GetWallRoot) false true)
  (Collision|SetCollisionEnabled (Variables|Default|Getwall) "NoCollision")
  (Utilities|FlowControl|DelayUntilNextTick)
  (Collision|SetCollisionResponsetoChannel (Variables|Default|Getdoorframeleft) "ECC_Visibility" "ECR_Ignore")
  (Collision|SetCollisionResponsetoChannel (Variables|Default|Getdoorframetop) "ECC_Visibility" "ECR_Ignore")
  (Collision|SetCollisionResponsetoChannel (Variables|Default|Getdoorframeright) "ECC_Visibility" "ECR_Ignore")
  (Collision|SetCollisionResponsetoChannel (Variables|Default|GetDoor) "ECC_Visibility" "ECR_Block")
  (Utilities|FlowControl|Delay 3.0)
  (CallFunction|OpenDoor))

(fn ConstructionScript)

(fn GetInteractionType
  (params (bIsCammy :type Boolean) (HitComponent :type Primitive%20Component%20Object%20Reference))
  (if (== HitComponent (Variables|Default|GetDoor))
    (return "NewEnumerator2" "")
    (else
      (return "NewEnumerator0" ""))))

(fn HoverOngoing
  (params (HeldItem :type Pickupable%20Interface%20Interface) (HitComponent :type Primitive%20Component%20Object%20Reference))
  (return false))

(fn HoverStart
  (params (HeldItem :type Pickupable%20Interface%20Interface) (HitComponent :type Primitive%20Component%20Object%20Reference) (bIsCammy :type Boolean))
  (return false))