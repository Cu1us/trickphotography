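; Wire cutters pickup, a big held item with its own held transform and scale, built on a parent pickup Blueprint.
; Non-Cammy pickup plays a grab sound and switches the three meshes to first-person rendering without shadows.
; Dropping restores rendering and scale, then re-enables blocking against world channels on the root after a short delay.
; PlayAnim runs a timeline that pitches the Right mesh for the clipping motion.
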(event Custom|PlayAnim
  (bind _rot (Timeline|Clip PlayFromStart)
    (:Update
      (Transformation|SetRelativeRotation (Variables|Default|GetRight) (Math|Rotator|MakeRotator 0.0 _rot 0.0) false false))))

(event EventBeginPlay
  (|CallParentFunction)
  (Utilities|FlowControl|DelayUntilNextTick)
  (Physics|SetSimulatePhysics (Variables|Default|GetCube) false))

(event Collision|EventActorBeginOverlap
  (params (OtherActor :type Actor%20Object%20Reference)))

(event EventTick
  (params (DeltaSeconds :type Float%20%28single-precision%29)))

(event EventOnPickup
  (params (isCammy :type Boolean))
  (|CallParentFunction isCammy)
  (if (not isCammy)
    (Audio|PlaySoundatLocation "/Game/TrickPhotography/Audio/Generic/SFX_GrabCutters.SFX_GrabCutters" (Transformation|GetActorLocation) "0, 0, 0" 1.0 1.0 0.0 0 0 0 0)
    (CallFunction|FirstPersonMode true (Variables|Default|GetCube))
    (CallFunction|FirstPersonMode true (Variables|Default|GetRight))
    (CallFunction|FirstPersonMode true (Variables|Default|GetLeft))))

(event EventOnDrop
  (params (isCammy :type Boolean))
  (|CallParentFunction isCammy)
  (Transformation|SetWorldScale3D (Variables|Default|GetCube) "0.450000,0.450000,0.450000")
  (CallFunction|FirstPersonMode false (Variables|Default|GetCube))
  (CallFunction|FirstPersonMode false (Variables|Default|GetRight))
  (CallFunction|FirstPersonMode false (Variables|Default|GetLeft))
  (bind _asprimitive_component (Utilities|Casting|CastToPrimitiveComponent (Variables|Transformation|GetRootComponent)))
  (Utilities|FlowControl|Delay 0.3)
  (Collision|SetCollisionResponsetoChannel _asprimitive_component "ECC_WorldStatic" "ECR_Block")
  (Collision|SetCollisionResponsetoChannel _asprimitive_component "ECC_WorldDynamic" "ECR_Block"))

(fn ConstructionScript)

(fn CanbePickedUp
  (params (isCammy :type Boolean))
  (return true))

(fn GetPickupID
  (return (Variables|Default|GetPickupID)))

(fn FirstPersonMode
  (params (bFirstPersonMode :type Boolean) (Mesh :type Static%20Mesh%20Component%20Object%20Reference))
  (if bFirstPersonMode
    (Rendering|SetFirstPersonPrimitiveType Mesh "FirstPerson")
    (Rendering|SetCastShadow Mesh false)
    (else
      (Rendering|SetFirstPersonPrimitiveType Mesh "None")
      (Rendering|SetCastShadow Mesh true))))

(fn GetCustomTransforms
  (return (Variables|Default|GetHeld%20Transform) "" true true))

(fn GetInteractionType
  (params (bIsCammy :type Boolean) (HitComponent :type Primitive%20Component%20Object%20Reference))
  (return "NewEnumerator3" "Pick up wire cutters"))

(fn HoverOngoing
  (params (HeldItem :type Pickupable%20Interface%20Interface) (HitComponent :type Primitive%20Component%20Object%20Reference))
  (return true))

(fn HoverStart
  (params (HeldItem :type Pickupable%20Interface%20Interface) (HitComponent :type Primitive%20Component%20Object%20Reference) (bIsCammy :type Boolean))
  (return true))