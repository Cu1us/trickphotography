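; BP_PolaroidPack is a highlightable pickup that unlocks a camera filter when the player uses it.
; Pickup and drop toggle first-person rendering and shadow casting, with pickup skipping this for Cammy.
; UsePolaroid detaches the pack and moves it along the main character's SplineThrow via a timeline.
; It then unlocks FilterToUnlock, optionally puts a tutorial photo in the left hand, shows a video tutorial for one filter, and destroys itself.
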(event Custom|UsePolaroid
  (Variables|Default|SetRotation (Transformation|GetActorRotation))
  (Variables|Default|SetLocation (Transformation|GetActorLocation))
  (Transformation|DetachFromActor "KeepWorld" "KeepWorld" "KeepWorld")
  (bind _lerp (Timeline|Lerp Play)
    (:Update
      (Transformation|SetActorLocationAndRotation (.location (Spline|GetTransformatTime (Variables|/Game/TrickPhotography/Programmers/Core/Player/BP_MainCharacter.BP_MainCharacter_C|GetSplineThrow (Variables|Default|GetMain%20Char)) _lerp "World" false false)) (.rotation (Spline|GetTransformatTime (Variables|/Game/TrickPhotography/Programmers/Core/Player/BP_MainCharacter.BP_MainCharacter_C|GetSplineThrow (Variables|Default|GetMain%20Char)) _lerp "World" false false))))
    (:Finished
      (Default|FeedingPolaroid (Variables|Default|GetMain%20Char) false)
      (Default|UnlockNewFilter (Variables|Default|GetAs%20Main%20Player%20Controller) (Variables|Pickup|GetFilterToUnlock))
      (Utilities|IsValid (Variables|Default|GetTutorialMat)
        (:Is%20Valid
          (|SpawnTutorialObjectInPlayersHand (Variables|Default|GetAs%20Main%20Player%20Controller)))
        (:Is%20Not%20Valid
          _))
      (if (Utilities|Enum|Equal(Enum) (Variables|Pickup|GetFilterToUnlock) "NewEnumerator1")
        (Default|ShowVideoTutorialDelayed (Variables|Default|GetAs%20Main%20Player%20Controller) "/Game/TrickPhotography/Dialogue/Tutorials/DA_Tutorial_Filters.DA_Tutorial_Filters" 0.75))
      (Actor|DestroyActor))))

(event EventHoverEnd
  (params (HeldItem :type Pickupable%20Interface%20Interface) (bIsCammy :type Boolean))
  (Class|FilterActor|SetPPMHighlight (Variables|Default|GetDefaultPPM)))

(event EventBeginPlay
  (Class|FilterActor|SetPPMHighlight (Variables|Default|GetDefaultPPM))
  (Utilities|FlowControl|DelayUntilNextTick)
  (Physics|SetSimulatePhysics (Variables|Default|GetPack) false)
  (Utilities|FlowControl|Delay 1.0)
  (bind _asmain_player_controller (Utilities|Casting|CastToMainPlayerController (Game|GetPlayerController 0)))
  (bind _output_get (Variables|Default|SetAs%20Main%20Player%20Controller _asmain_player_controller))
  (Variables|Default|SetMain%20Char (Variables|/Game/TrickPhotography/Programmers/Core/Player/MainPlayerController.MainPlayerController_C|GetMainChar _output_get))
  (Variables|Default|SetCammy%20Char (Variables|/Game/TrickPhotography/Programmers/Core/Player/MainPlayerController.MainPlayerController_C|GetCammyChar _asmain_player_controller)))

(event EventTick
  (params (DeltaSeconds :type Float%20%28single-precision%29))
  (|CallParentFunction DeltaSeconds))

(event EventOnPickup
  (params (isCammy :type Boolean))
  (bind _pack (Variables|Default|GetPack))
  (|CallParentFunction isCammy)
  (if (not isCammy)
    (Rendering|SetFirstPersonPrimitiveType _pack "FirstPerson")
    (Rendering|SetCastShadow _pack false)))

(event EventActivate
  (params (cameraTransform :type Transform) (isCammy :type Boolean))
  (|CallParentFunction cameraTransform isCammy)
  (Variables|/Game/TrickPhotography/Programmers/Core/Player/BP_MainCharacter.BP_MainCharacter_C|SetbHoldingPolaroidPack (Variables|Default|GetMain%20Char) false))

(event EventOnDrop
  (params (isCammy :type Boolean))
  (|CallParentFunction isCammy)
  (Rendering|SetFirstPersonPrimitiveType (Variables|Default|GetPack) "None")
  (Rendering|SetCastShadow (Variables|Default|GetPack) true))

(fn ConstructionScript)

(fn GetCustomTransforms
  (return (Variables|Default|GetHeld%20Transform) (Variables|Default|GetLook%20at%20Transform) false false))

(fn GetInteractionType
  (params (bIsCammy :type Boolean) (HitComponent :type Primitive%20Component%20Object%20Reference))
  (return "NewEnumerator0" ""))

(fn HoverOngoing
  (params (HeldItem :type Pickupable%20Interface%20Interface) (HitComponent :type Primitive%20Component%20Object%20Reference))
  (return false))

(fn HoverStart
  (params (HeldItem :type Pickupable%20Interface%20Interface) (HitComponent :type Primitive%20Component%20Object%20Reference) (bIsCammy :type Boolean))
  (Class|FilterActor|SetPPMHighlight "HighlightPickup")
  (return false))