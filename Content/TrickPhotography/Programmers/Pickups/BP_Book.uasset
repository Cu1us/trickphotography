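; Pickup book that the player carries and places into BP_BookSlot actors.
; Activate multi-traces forward from the camera, and on hitting a slot detaches the book from the player, snaps and attaches it, and registers its PickupID.
; Pickup clears any attached slot's registration, otherwise enabling first-person rendering when not Cammy.
; Drop resets rendering and scale, then restores world-blocking collision after a short delay; hover toggles a highlight.
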(event EventActivate
  (params (cameraTransform :type Transform) (isCammy :type Boolean))
  (bind (_outhits _returnvalue) (Class|KismetSystemLibrary|LineTraceMultibyProfile (.location cameraTransform) (+ (.location cameraTransform) (* (Math|Vector|GetForwardVector (.rotation cameraTransform)) (Math|Float|MakeLiteralFloat 7.5e+02))) "BlockAll" false (Utilities|Array|MakeArray (Game|GetPlayerCharacter 0)) "ForDuration" true "(R=1.000000,G=0.000000,B=0.000000,A=1.000000)" "(R=0.000000,G=1.000000,B=0.000000,A=1.000000)" 1.0))
  (if _returnvalue
    (bind _array_element (Utilities|Array|ForEachLoopwithBreak _outhits :!label _label)
      (:LoopBody
        (bind _asbp_book_slot (Utilities|Casting|CastToBP_BookSlot (.HitActor (Collision|BreakHitResult _array_element))))
        (bind _asbp_main_character (Utilities|Casting|CastToBP_MainCharacter (Game|GetPlayerCharacter 0)))
        (Default|DetachHeldObject _asbp_main_character)
        (Transformation|SetWorldLocationAndRotation (Variables|Default|GetBook) (.location (Transformation|GetActorTransform _asbp_book_slot)) (.rotation (Transformation|GetActorTransform _asbp_book_slot)) false true)
        (Development|PrintString "ya")
        (Class|PickupableInterface|OnDrop false)
        (Physics|SetSimulatePhysics (Variables|Default|GetBook) false)
        (Transformation|SetActorScale3D "1.000000,1.000000,1.000000")
        (Transformation|AttachActorToActor _asbp_book_slot "" "KeepWorld" "KeepWorld" "KeepWorld" true)
        (Default|SetRegisteredBook _asbp_book_slot (Variables|Default|GetPickupID))
        (Variables|Default|SetAttachedSlot _asbp_book_slot)
        (goto _label Break)))))

(event EventOnPickup
  (params (isCammy :type Boolean))
  (|CallParentFunction isCammy)
  (Utilities|IsValid (Variables|Default|GetAttachedSlot)
    (:Is%20Valid
      (Default|SetRegisteredBook (Variables|Default|GetAttachedSlot))
      (Variables|Default|SetAttachedSlot 0))
    (:Is%20Not%20Valid
      (if (not isCammy)
        (Rendering|SetFirstPersonPrimitiveType (Variables|Default|GetBook) "FirstPerson")))))

(event EventHoverEnd
  (params (HeldItem :type Pickupable%20Interface%20Interface) (bIsCammy :type Boolean))
  (Class|FilterActor|SetPPMHighlight "None"))

(event EventOnThermalPhoto)

(event EventOnDrop
  (params (isCammy :type Boolean))
  (|CallParentFunction isCammy)
  (Rendering|SetFirstPersonPrimitiveType (Variables|Default|GetBook) "None")
  (Transformation|SetActorScale3D "1.000000,1.000000,1.000000")
  (bind _asprimitive_component (Utilities|Casting|CastToPrimitiveComponent (Variables|Transformation|GetRootComponent)))
  (Utilities|FlowControl|Delay 0.3)
  (Collision|SetCollisionResponsetoChannel _asprimitive_component "ECC_WorldStatic" "ECR_Block")
  (Collision|SetCollisionResponsetoChannel _asprimitive_component "ECC_WorldDynamic" "ECR_Block"))

(fn ConstructionScript)

(fn GetCustomTransforms
  (return (Variables|Default|GetHeld%20Transform) "" true true))

(fn GetInteractionType
  (params (bIsCammy :type Boolean) (HitComponent :type Primitive%20Component%20Object%20Reference))
  (return "NewEnumerator3" ""))

(fn HoverOngoing
  (params (HeldItem :type Pickupable%20Interface%20Interface) (HitComponent :type Primitive%20Component%20Object%20Reference))
  (return false))

(fn HoverStart
  (params (HeldItem :type Pickupable%20Interface%20Interface) (HitComponent :type Primitive%20Component%20Object%20Reference) (bIsCammy :type Boolean))
  (Class|FilterActor|SetPPMHighlight "HighlightPickup")
  (return false))