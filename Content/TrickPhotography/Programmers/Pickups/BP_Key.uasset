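; BP_Key is a key pickup the player can highlight on hover, pick up, hold and drop, built on a parent pickup class.
; Hover toggles a PPM highlight, and interaction functions supply the held transform and interaction type.
; When picked up by anyone other than Cammy, the key renders as a first-person primitive without shadow.
; Dropping restores normal rendering, then re-enables blocking against world static and dynamic objects after a short delay.
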(event EventBeginPlay
  (|CallParentFunction)
  (Utilities|FlowControl|DelayUntilNextTick)
  (Physics|SetSimulatePhysics (Variables|Default|GetKey) false))

(event Collision|EventActorBeginOverlap
  (params (OtherActor :type Actor%20Object%20Reference)))

(event EventTick
  (params (DeltaSeconds :type Float%20%28single-precision%29)))

(event EventHoverEnd
  (params (HeldItem :type Pickupable%20Interface%20Interface) (bIsCammy :type Boolean))
  (Class|FilterActor|SetPPMHighlight "None"))

(event EventOnDrop
  (params (isCammy :type Boolean))
  (bind _key (Variables|Default|GetKey))
  (|CallParentFunction isCammy)
  (Rendering|SetCastShadow _key true)
  (Rendering|SetFirstPersonPrimitiveType _key "None")
  (bind _asprimitive_component (Utilities|Casting|CastToPrimitiveComponent (Variables|Transformation|GetRootComponent)))
  (Utilities|FlowControl|Delay 0.3)
  (Collision|SetCollisionResponsetoChannel _asprimitive_component "ECC_WorldStatic" "ECR_Block")
  (Collision|SetCollisionResponsetoChannel _asprimitive_component "ECC_WorldDynamic" "ECR_Block"))

(event EventOnPickup
  (params (isCammy :type Boolean))
  (bind _key (Variables|Default|GetKey))
  (|CallParentFunction isCammy)
  (if (not isCammy)
    (Rendering|SetFirstPersonPrimitiveType _key "FirstPerson")
    (Rendering|SetCastShadow _key false)))

(fn ConstructionScript)

(fn GetCustomTransforms
  (return (Variables|Default|GetHeld%20Transform) "" false false))

(fn GetInteractionType
  (params (bIsCammy :type Boolean) (HitComponent :type Primitive%20Component%20Object%20Reference))
  (return "NewEnumerator3" ""))

(fn HoverOngoing
  (params (HeldItem :type Pickupable%20Interface%20Interface) (HitComponent :type Primitive%20Component%20Object%20Reference))
  (return false))

(fn HoverStart
  (params (HeldItem :type Pickupable%20Interface%20Interface) (HitComponent :type Primitive%20Component%20Object%20Reference) (bIsCammy :type Boolean))
  (Class|FilterActor|SetPPMHighlight "HighlightPickup")
  (return true))