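; BP_CammyPickup is a pickup that unlocks Cammy for the player.
; On pickup it runs the parent logic, then calls UnlockCammy on the main player controller with a tutorial material.
; A tick later it force-drops the held object with destroy set, then destroys itself.
; Hover start and end toggle the post-process pickup highlight.
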(event EventBeginPlay)

(event Collision|EventActorBeginOverlap
  (params (OtherActor :type Actor%20Object%20Reference)))

(event EventTick
  (params (DeltaSeconds :type Float%20%28single-precision%29)))

(event EventOnPickup
  (params (isCammy :type Boolean))
  (|CallParentFunction isCammy)
  (bind _asmain_player_controller (Utilities|Casting|CastToMainPlayerController (Game|GetPlayerController 0)))
  (Default|UnlockCammy _asmain_player_controller (Variables|Default|GetTutorialMat))
  (Utilities|FlowControl|DelayUntilNextTick)
  (Default|DropObject (Variables|/Game/TrickPhotography/Programmers/Core/Player/MainPlayerController.MainPlayerController_C|GetMainChar _asmain_player_controller) true true)
  (Actor|DestroyActor))

(event EventHoverEnd
  (params (HeldItem :type Pickupable%20Interface%20Interface) (bIsCammy :type Boolean))
  (Class|FilterActor|SetPPMHighlight "None"))

(fn ConstructionScript)

(fn GetInteractionType
  (params (bIsCammy :type Boolean) (HitComponent :type Primitive%20Component%20Object%20Reference))
  (return "NewEnumerator0" ""))

(fn HoverOngoing
  (params (HeldItem :type Pickupable%20Interface%20Interface) (HitComponent :type Primitive%20Component%20Object%20Reference))
  (return false))

(fn HoverStart
  (params (HeldItem :type Pickupable%20Interface%20Interface) (HitComponent :type Primitive%20Component%20Object%20Reference) (bIsCammy :type Boolean))
  (Class|FilterActor|SetPPMHighlight "HighlightPickup")
  (return false))