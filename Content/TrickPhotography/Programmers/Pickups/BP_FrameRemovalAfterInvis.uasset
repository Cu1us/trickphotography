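; Pickup Blueprint for a frame that starts with physics and collision off until UnlockMoveable enables its collision and destroys the associated Box.
; Only the non-Cammy player can hover or pick it up.
; Pickup renders the frame as a first-person primitive.
; Drop clears that, then after a short delay sets the root to block WorldStatic and WorldDynamic.
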(event Custom|UnlockMoveable
  (bind _box (Variables|Default|GetBox))
  (Collision|SetCollisionEnabled (Variables|Default|GetFrame) "QueryAndPhysics")
  (Utilities|IsValid _box
    (:Is%20Valid
      (Actor|DestroyActor _box))))

(event EventBeginPlay
  (|CallParentFunction)
  (Utilities|FlowControl|DelayUntilNextTick)
  (Physics|SetSimulatePhysics (Variables|Default|GetFrame) false)
  (Collision|SetCollisionEnabled (Variables|Default|GetFrame) "NoCollision"))

(event Collision|EventActorBeginOverlap
  (params (OtherActor :type Actor%20Object%20Reference)))

(event EventTick
  (params (DeltaSeconds :type Float%20%28single-precision%29)))

(event EventOnDrop
  (params (isCammy :type Boolean))
  (|CallParentFunction isCammy)
  (Rendering|SetFirstPersonPrimitiveType (Variables|Default|GetFrame) "None")
  (bind _asprimitive_component (Utilities|Casting|CastToPrimitiveComponent (Variables|Transformation|GetRootComponent)))
  (Utilities|FlowControl|Delay 0.3)
  (Collision|SetCollisionResponsetoChannel _asprimitive_component "ECC_WorldStatic" "ECR_Block")
  (Collision|SetCollisionResponsetoChannel _asprimitive_component "ECC_WorldDynamic" "ECR_Block"))

(event EventOnPickup
  (params (isCammy :type Boolean))
  (|CallParentFunction isCammy)
  (if (not isCammy)
    (Rendering|SetFirstPersonPrimitiveType (Variables|Default|GetFrame) "FirstPerson")))

(fn ConstructionScript)

(fn CanbePickedUp
  (params (isCammy :type Boolean))
  (if isCammy
    (return false)
    (else
      (return true))))

(fn GetInteractionType
  (params (bIsCammy :type Boolean) (HitComponent :type Primitive%20Component%20Object%20Reference))
  (return "NewEnumerator3" ""))

(fn HoverOngoing
  (params (HeldItem :type Pickupable%20Interface%20Interface) (HitComponent :type Primitive%20Component%20Object%20Reference))
  (return false))

(fn HoverStart
  (params (HeldItem :type Pickupable%20Interface%20Interface) (HitComponent :type Primitive%20Component%20Object%20Reference) (bIsCammy :type Boolean))
  (if bIsCammy
    (return false)
    (else
      (return true))))