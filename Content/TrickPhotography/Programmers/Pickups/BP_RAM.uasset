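; BP_RAM is a pickup item for a RAM component that players can always pick up and carry as a small held item.
; Pickup switches the mesh to first-person rendering without shadows, and drop reverses both.
; After a drop, a short delay precedes setting the root component to block static and dynamic world objects.
; Hover handlers return false, and pickup ID comes from the parent class.
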(event EventBeginPlay)

(event Collision|EventActorBeginOverlap
  (params (OtherActor :type Actor%20Object%20Reference)))

(event EventTick
  (params (DeltaSeconds :type Float%20%28single-precision%29)))

(event EventOnPickup
  (params (isCammy :type Boolean))
  (|CallParentFunction isCammy)
  (Rendering|SetFirstPersonPrimitiveType (Variables|Default|GetRAM) "FirstPerson")
  (Rendering|SetCastShadow (Variables|Default|GetRAM) false))

(event EventOnDrop
  (params (isCammy :type Boolean))
  (|CallParentFunction isCammy)
  (Rendering|SetFirstPersonPrimitiveType (Variables|Default|GetRAM) "None")
  (Rendering|SetCastShadow (Variables|Default|GetRAM) true)
  (bind _asprimitive_component (Utilities|Casting|CastToPrimitiveComponent (Variables|Transformation|GetRootComponent)))
  (Utilities|FlowControl|Delay 0.3)
  (Collision|SetCollisionResponsetoChannel _asprimitive_component "ECC_WorldStatic" "ECR_Block")
  (Collision|SetCollisionResponsetoChannel _asprimitive_component "ECC_WorldDynamic" "ECR_Block"))

(fn ConstructionScript)

(fn GetPickupID
  (bind _returnvalue (|CallParentFunction))
  (return _returnvalue))

(fn CanbePickedUp
  (params (isCammy :type Boolean))
  (return true))

(fn GetCustomTransforms
  (return (Variables|Default|GetHeld%20Transform) "" false false))

(fn GetInteractionType
  (params (bIsCammy :type Boolean) (HitComponent :type Primitive%20Component%20Object%20Reference))
  (return "NewEnumerator3" ""))

(fn HoverOngoing
  (params (HeldItem :type Pickupable%20Interface%20Interface) (HitComponent :type Primitive%20Component%20Object%20Reference))
  (return false))

(fn HoverStart
  (params (HeldItem :type Pickupable%20Interface%20Interface) (HitComponent :type Primitive%20Component%20Object%20Reference) (bIsCammy :type Boolean))
  (return false))