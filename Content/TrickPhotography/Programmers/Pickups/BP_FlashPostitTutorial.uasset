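; BP_FlashPostitTutorial is a small pickup item that can be held and dropped, apparently a tutorial post-it.
; On pickup by a non-Cammy holder, its FilterStaticMesh switches to first-person primitive rendering and stops casting shadows.
; Dropping restores normal rendering and shadows, then after a short delay sets the root to block world static and dynamic channels.
; Interface overrides supply the held transform and a fixed interaction type, while hover checks return false.
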(event EventBeginPlay)

(event Collision|EventActorBeginOverlap
  (params (OtherActor :type Actor%20Object%20Reference)))

(event EventTick
  (params (DeltaSeconds :type Float%20%28single-precision%29)))

(event EventOnDrop
  (params (isCammy :type Boolean))
  (|CallParentFunction isCammy)
  (Rendering|SetFirstPersonPrimitiveType (Variables|Default|GetFilterStaticMesh) "None")
  (Rendering|SetCastShadow (Variables|Default|GetFilterStaticMesh) true)
  (bind _asprimitive_component (Utilities|Casting|CastToPrimitiveComponent (Variables|Transformation|GetRootComponent)))
  (Utilities|FlowControl|Delay 0.3)
  (Collision|SetCollisionResponsetoChannel _asprimitive_component "ECC_WorldStatic" "ECR_Block")
  (Collision|SetCollisionResponsetoChannel _asprimitive_component "ECC_WorldDynamic" "ECR_Block"))

(event EventOnPickup
  (params (isCammy :type Boolean))
  (bind _filterstaticmesh (Variables|Default|GetFilterStaticMesh))
  (|CallParentFunction isCammy)
  (if (not isCammy)
    (Rendering|SetFirstPersonPrimitiveType _filterstaticmesh "FirstPerson")
    (Rendering|SetCastShadow _filterstaticmesh false)))

(fn ConstructionScript)

(fn GetCustomTransforms
  (return (Variables|Default|GetHeld%20Transform) "" false false))

(fn GetInteractionType
  (params (bIsCammy :type Boolean) (HitComponent :type Primitive%20Component%20Object%20Reference))
  (return "NewEnumerator0" ""))

(fn HoverOngoing
  (params (HeldItem :type Pickupable%20Interface%20Interface) (HitComponent :type Primitive%20Component%20Object%20Reference))
  (return false))

(fn HoverStart
  (params (HeldItem :type Pickupable%20Interface%20Interface) (HitComponent :type Primitive%20Component%20Object%20Reference) (bIsCammy :type Boolean))
  (return false))