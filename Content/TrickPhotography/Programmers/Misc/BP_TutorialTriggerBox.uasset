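; BP_TutorialTriggerBox is a one-shot trigger volume that shows a video tutorial through MainPlayerController when an allowed character overlaps it.
; Flags select BP_MainCharacter or BP_CammyCharacter as the triggering character, with the Cammy flag checked only when the player flag is off.
; CanBeTriggered gates the overlap but always returns true here.
; The construction script sizes the box from BoxSize, clamped to non-negative values.
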(event Collision|EventActorBeginOverlap
  (params (OtherActor :type Actor%20Object%20Reference))
  (bind _triggable (CallFunction|CanbeTriggered))
  (if _triggable
    (if (not (Variables|Default|GetbHasBeenTriggered))
      (Utilities|IsValid (Variables|Tutorial|GetTutorialToShow)
        (:Is%20Valid
          (if (Variables|Tutorial|GetbTriggableByPlayer)
            (Utilities|Casting|CastToBP_MainCharacter OtherActor)
            (bind _asmain_player_controller (Utilities|Casting|CastToMainPlayerController (Game|GetPlayerController 0) :!label _label))
            (Default|ShowVideoTutorial _asmain_player_controller (Variables|Tutorial|GetTutorialToShow))
            (Variables|Default|SetbHasBeenTriggered true)
            (elif (Variables|Tutorial|GetbTriggableByCammy)
              (Utilities|Casting|CastToBP_CammyCharacter OtherActor)
              (goto _label))))))))

(fn ConstructionScript
  (bind _output_get (Variables|Default|SetBoxSize (Math|Vector|MakeVector (Math|Float|Max(Float) (.x (stale _output_get)) 0.0) (Math|Float|Max(Float) (.y (stale _output_get)) 0.0) (Math|Float|Max(Float) (.z (stale _output_get)) 0.0))))
  (Components|Box|SetBoxExtent (Variables|Default|GetTriggerBox) (Variables|Default|GetBoxSize) false))

(fn CanbeTriggered
  (return (Class|KismetSystemLibrary|MakeLiteralBool true)))